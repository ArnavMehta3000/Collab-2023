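; BP_Train is an environment train actor that moves between two points using an InterpToMovement component.
; The construction script builds two relative control points from the A and B variables and sets the travel time from Duration.
; Any actor overlap plays a 2D sound, with no filtering on the overlapping actor.
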(event EventBeginPlay)

(event Collision|EventActorBeginOverlap
  (params (OtherActor :type Actor%20Object%20Reference))
  (Audio|PlaySound2D 0 1.0 1.0 0.0 0 0))

(event EventTick
  (params (DeltaSeconds :type Float%20%28single-precision%29)))

(fn ConstructionScript
  (bind _interptomovement (Variables|Default|GetInterpToMovement))
  (Variables|/Script/Engine.InterpToMovementComponent|SetControlPoints _interptomovement (Utilities|Array|MakeArray (Utilities|Struct|MakeInterpControlPoint (Variables|Default|GetA) true) (Utilities|Struct|MakeInterpControlPoint (Variables|Default|GetB) true)))
  (Variables|/Script/Engine.InterpToMovementComponent|SetDuration _interptomovement (Variables|Default|GetDuration)))