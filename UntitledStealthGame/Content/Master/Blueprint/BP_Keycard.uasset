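; BP_Keycard is a keycard pickup that grants the player access by flagging that they hold it.
; When its Sphere overlaps a BP_MasterPlayer, it sets that player's HasKeycard to true, then destroys itself after a brief delay.
; An Initialize event prints the keycard's position and name to the screen as debug output.
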(event OnComponentBeginOverlap(Sphere)
  (params (OverlappedComponent :type Primitive%20Component%20Object%20Reference) (OtherActor :type Actor%20Object%20Reference) (OtherComp :type Primitive%20Component%20Object%20Reference) (OtherBodyIndex :type Integer) (bFromSweep :type Boolean) (SweepResult :type Hit%20Result%20Structure%20%28by%20ref%29))
  (bind _asbp_master_player (Utilities|Casting|CastToBP_MasterPlayer OtherActor))
  (Variables|/Game/Master/Blueprint/Player/BP_MasterPlayer.BP_MasterPlayer_C|SethasKeycard _asbp_master_player true)
  (Utilities|FlowControl|Delay 0.1)
  (Actor|DestroyActor))

(event EventInitialize
  (Development|PrintString (Utilities|String|Append "Init Key at position: " (Utilities|String|ToString(Vector) (Transformation|GetActorLocation)) " Name: " (Utilities|GetDisplayName self)) true true "(R=0.000000,G=1.000000,B=0.156293,A=1.000000)" 2e+01))

(fn ConstructionScript)