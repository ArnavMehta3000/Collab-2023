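; BP_LevelSwitcher is a trigger actor that moves the game to another level when BP_MasterPlayer overlaps its Box.
; On overlap it shows a LoadingScreen widget, waits a short random delay, opens the ToOpen level with OptionsString, then removes the widget.
; SetGenCount writes a count into OptionsString as a "GEN=" option, passing it to the opened level, and prints the string.
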(event OnComponentBeginOverlap(Box)
  (params (OverlappedComponent :type Primitive%20Component%20Object%20Reference) (OtherActor :type Actor%20Object%20Reference) (OtherComp :type Primitive%20Component%20Object%20Reference) (OtherBodyIndex :type Integer) (bFromSweep :type Boolean) (SweepResult :type Hit%20Result%20Structure%20%28by%20ref%29))
  (Utilities|Casting|CastToBP_MasterPlayer OtherActor)
  (bind _returnvalue (UserInterface|CreateWidget "/Game/Master/Blueprint/UI/LoadingScreen.LoadingScreen_C"))
  (UserInterface|Viewport|AddtoViewport _returnvalue 0)
  (Utilities|FlowControl|Delay (Math|Random|RandomFloatinRange 1.23 3.4))
  (Game|OpenLevel(byObjectReference) (Variables|Default|GettoOpen) true (Variables|Default|GetoptionsString))
  (Widget|RemovefromParent _returnvalue))

(fn ConstructionScript)

(fn SetGenCount
  (params (count :type Integer))
  (bind _output_get (Variables|Default|SetoptionsString (Utilities|String|Append "GEN=" (Utilities|String|ToString(Integer) count))))
  (Development|PrintString _output_get))