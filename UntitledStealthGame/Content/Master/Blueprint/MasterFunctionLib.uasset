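; Blueprint function library with two helpers that start and stop climbing for player 0's character, given an overlapping or other actor.
; Starting requires a 500-unit visibility trace along the camera's forward vector to hit anything, then zeroes velocity and switches movement to Flying.
; Stopping switches movement to Falling without a trace.
; The trace leaves persistent debug drawing and does not check what it hit.
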(fn OnTryStartClimb
  (params (otherActor :type Actor%20Object%20Reference))
  (bind _returnvalue (Game|GetPlayerCharacter 0))
  (bind _returnvalue_2 (Game|GetPlayerCameraManager 0))
  (bind _returnvalue_3 (Camera|GetCameraLocation _returnvalue_2))
  (bind _charactermovement (Variables|/Script/Engine.Character|GetCharacterMovement _returnvalue))
  (if (== otherActor (Game|GetPlayerCharacter 0))
    (bind _returnvalue_4 (Collision|LineTraceByChannel 0 _returnvalue_3 (+ _returnvalue_3 (* (Transformation|GetActorForwardVector _returnvalue_2) 5e+02)) "TraceTypeQuery1" false 0 "Persistent" false "(R=1.000000,G=0.000000,B=0.000000,A=1.000000)" "(R=0.000000,G=1.000000,B=0.000000,A=1.000000)" 2.0))
    (if _returnvalue_4
      (Variables|/Script/Engine.MovementComponent|SetVelocity _charactermovement "0, 0, 0")
      (Pawn|Components|CharacterMovement|SetMovementMode _charactermovement "MOVE_Flying" 0))))

(fn OnTryStopClimb
  (params (otherActor :type Actor%20Object%20Reference))
  (bind _returnvalue (Game|GetPlayerCharacter 0))
  (if (== otherActor _returnvalue)
    (Pawn|Components|CharacterMovement|SetMovementMode (Variables|/Script/Engine.Character|GetCharacterMovement _returnvalue) "MOVE_Falling" 0)))