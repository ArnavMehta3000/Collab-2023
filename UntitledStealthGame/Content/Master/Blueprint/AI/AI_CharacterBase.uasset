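; Base AI character Blueprint that reacts to state changes from its AIC_MasterAiController.
; Initialize casts and stores the controller, then binds to its state-change event.
; Each change updates StateText, with Return labelled as Wander, and routes the state through UpdateSpeedByState.
; The SetSpeed macro has one input per state, sets the matching MaxWalkSpeed and prints it for debugging.
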(event Custom|OnAiStateChange_Event
  (params (newState :type E_EnemyStates%20Enum :default "NewEnumerator0"))
  (Rendering|Components|TextRender|SetText (Variables|Default|GetState%20Text) (Utilities|Select :Index newState :NewEnumerator0 (Utilities|Text|MakeLiteralText "Wander") :NewEnumerator1 (Utilities|Text|MakeLiteralText "Investigate") :NewEnumerator5 (Utilities|Text|MakeLiteralText "Search") :NewEnumerator2 (Utilities|Text|MakeLiteralText "Chase") :NewEnumerator3 (Utilities|Text|MakeLiteralText "Attack") :NewEnumerator4 (Utilities|Text|MakeLiteralText "Wander")))
  (CallFunction|UpdateSpeedbyState newState))

(event EventInitialize
  (bind _asaic_master_ai_controller (Utilities|Casting|CastToAIC_MasterAiController (Pawn|GetController)))
  (bind _output_get (Variables|Default|SetaiController _asaic_master_ai_controller))
  (EventDispatchers|AssignOnAiStateChange _output_get (delegate Custom|OnAiStateChange_Event)))

(fn ConstructionScript)

(fn UpdateSpeedbyState
  (params (newState :type E_EnemyStates%20Enum :default "NewEnumerator0"))
  (switch Utilities|FlowControl|Switch|SwitchonE_EnemyStates newState
    (:NewEnumerator0
      (Utilities|SetSpeed 2.5e+02 3e+02 5e+02 5e+02 2.5e+02 2.5e+02 :!label _label))
    (:NewEnumerator1
      (goto _label Investigate))
    (:NewEnumerator5
      (goto _label Search))
    (:NewEnumerator2
      (goto _label Chase))
    (:NewEnumerator3
      (goto _label Attack))
    (:NewEnumerator4
      (goto _label Return))))