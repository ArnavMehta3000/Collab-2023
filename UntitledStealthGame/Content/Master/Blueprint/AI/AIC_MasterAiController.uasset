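; Base AI controller that drives wander and investigate states for enemies through Blackboard values and state-change calls.
; Initialize caches the current room from the run game mode, seeds the Blackboard and runs an EQS query whose random results become wander points.
; Perception updates from the player switch to investigate on hearing; the sight check leads nowhere, leaving the chase switch unused.
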(event OnTargetPerceptionUpdated(AIPerception)
  (params (Actor :type Actor%20Object%20Reference) (Stimulus :type AI%20Stimulus%20Structure))
  (Utilities|ToMasterPlayer Actor
    (:then
      (bind _returnvalue (Class|AIPerceptionSystem|GetSenseClassforStimulus Stimulus))
      (Utilities|CheckforAiSenseClass _returnvalue "/Script/AIModule.AISense_Hearing"
        (:True
          (CallFunction|SwitchtoInvestigate Stimulus))
        (:False
          (Utilities|CheckforAiSenseClass _returnvalue "/Script/AIModule.AISense_Sight"))))))

(event Custom|SwitchToChase
  (params (stimulus :type AI%20Stimulus%20Structure))
  (bind (_blackboard _varout) (Utilities|SetBlackboardValues "state"))
  (bind (_blackboard_2 _varout_2) (Utilities|SetBlackboardValues "targetLocation"))
  (bind (_blackboard_3 _varout_3) (Utilities|SetBlackboardValues "isPlayerInSight"))
  (AI|Components|Blackboard|SetValueasEnum _blackboard _varout 2) ; Investigate state is 1
  (AI|Components|Blackboard|SetValueasBool _blackboard_3 _varout_3 true)
  (AI|Components|Blackboard|SetValueasVector _blackboard_2 _varout_2 (.stimuluslocation stimulus))
  (Default|CallOnAiStateChange "NewEnumerator2"))

(event Custom|OnQueryFinishedEvent_Event
  (params (QueryInstance :type Env%20Query%20Instance%20Blueprint%20Wrapper%20Object%20Reference) (QueryStatus :type EEnvQueryStatus%20Enum :default "Processing"))
  (CallFunction|GetWanderPointsfromEQS QueryInstance 7))

(event Custom|SwitchToInvestigate
  (params (stimulus :type AI%20Stimulus%20Structure))
  (bind (_blackboard _varout) (Utilities|SetBlackboardValues "investigateLocation"))
  (bind (_blackboard_2 _varout_2) (Utilities|SetBlackboardValues "state"))
  (AI|Components|Blackboard|SetValueasEnum _blackboard_2 _varout_2 1) ; Investigate state is 1
  (AI|Components|Blackboard|SetValueasVector _blackboard _varout (.stimuluslocation stimulus))
  (Default|CallOnAiStateChange "NewEnumerator1"))

(event EventInitialize
  (bind _asgm_run (Utilities|CaptureRunGameMode)
    (:Success
      (bind _output_get (Variables|Default|SetrunGameMode _asgm_run))
      (Variables|Default|SetselfRoom (Default|GetCurrentRoom _output_get)))
    (:Fail
      (Development|PrintString "AI CONTROLLER: FAILED TO CAST TO RUN GAME MODE" true true "(R=1.000000,G=0.000000,B=0.203612,A=1.000000)" 1e+01)))
  (CallFunction|InitBlackboard)
  (bind _returnvalue (AI|EQS|RunEQSQuery "/Game/Master/Blueprint/AI/BehaviourTrees/EQS_Queries/EQS_AI_FindWanderPoints.EQS_AI_FindWanderPoints" self "AllMatching"))
  (EventDispatchers|AssignOnQueryFinishedEvent _returnvalue (delegate Custom|OnQueryFinishedEvent_Event)))

(fn ConstructionScript)

(fn InitBlackboard
  (bind (_blackboard _varout) (Utilities|SetBlackboardValues "origin"))
  (bind (_blackboard_2 _varout_2) (Utilities|SetBlackboardValues "state"))
  (bind (_blackboard_3 _varout_3) (Utilities|SetBlackboardValues "wanderRadius"))
  (bind (_blackboard_4 _varout_4) (Utilities|SetBlackboardValues "investigateTime"))
  (AI|Components|Blackboard|SetValueasEnum _blackboard_2 _varout_2) ; Set State
  (AI|Components|Blackboard|SetValueasVector _blackboard _varout (Transformation|GetActorLocation)) ; Set Origin
  (AI|Components|Blackboard|SetValueasFloat _blackboard_3 _varout_3 (Variables|Blackboard|GetwanderRadius))
  (AI|Components|Blackboard|SetValueasFloat _blackboard_4 _varout_4 (Variables|Blackboard|GetinvestigateTime)))

(fn GetWanderPointsfromEQS
  (params (queryInstance :type Env%20Query%20Instance%20Blueprint%20Wrapper%20Object%20Reference) (pointCount :type Integer))
  (bind (_resultlocations _returnvalue) (AI|EQS|GetQueryResultsasLocations queryInstance))
  (if _returnvalue
    (for _index (range 0 pointCount)
      (bind _output_get (Variables|Default|Setpos (.OutItem (Utilities|Array|Random _resultlocations))))
      (Utilities|Array|AddUnique (Variables|Default|GetwanderPoints) _output_get))
    (Default|CallOnAiStateChange "NewEnumerator0")
    (return _returnvalue)
    (else
      (return _returnvalue))))