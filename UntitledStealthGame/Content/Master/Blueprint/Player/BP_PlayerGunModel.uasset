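; Player gun model Blueprint that handles shooting effects and hitscan damage.
; PlayShootMontage adds audio, traces from the fire point toward the camera's aim, applies damage and plays the gun's fire montage.
; Start/StopShooting toggle IsFiring, which gates a separate FireBullet function that spends ammo on a debug-drawn trace from the parent character's camera; nothing here calls it.
; Reload is an unfinished stub with disconnected ammo math.
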(event Custom|Stop%20Shooting
  (Variables|Default|SetisFiring false))

(event Custom|PlayShootMontage
  ;[1 1 1] Anim
  (AddComponent|AddAudioComponent false)
  ;[1 1 1] Line Trace
  (bind _outhit (Collision|LineTraceByChannel (Transformation|GetWorldLocation (Variables|Default|GetFirePoint)) (+ (Transformation|GetWorldLocation (stale Custom|Start%20Shooting Camera)) (* (Math|Vector|GetForwardVector (stale Custom|Start%20Shooting Camera)) 5e+03)) "TraceTypeQuery2" false 0 "None"))
  (Game|Damage|ApplyDamage (.hitactor _outhit) 2e+01 0 0)
  (Animation|Montage|PlayMontage (Variables|Default|GetGunModel) "/Game/Animation/Billy/ArmRig/Animations/GunAnimations/GunFire.GunFire"))

(event Custom|Start%20Shooting
  (params (Camera :type Camera%20Component%20Object%20Reference))
  (Variables|Default|SetisFiring true))

(fn ConstructionScript)

(fn FireBullet
  (if (Variables|Default|GetIsFiring)
    (bind _asbp_first_person_character (Utilities|Casting|CastToBP_FirstPersonCharacter (Actor|GetParentActor)))
    (if (> (Variables|Default|GetCurrentAmmo) 0)
      (bind _outhit (Collision|LineTraceByChannel (Transformation|GetWorldLocation (Variables|/Game/FirstPerson/Blueprints/BP_FirstPersonCharacter.BP_FirstPersonCharacter_C|GetFirstPersonCamera _asbp_first_person_character)) (+ (Transformation|GetWorldLocation (Variables|/Game/FirstPerson/Blueprints/BP_FirstPersonCharacter.BP_FirstPersonCharacter_C|GetFirstPersonCamera _asbp_first_person_character)) (* (Math|Vector|GetForwardVector (Transformation|GetWorldRotation (Variables|/Game/FirstPerson/Blueprints/BP_FirstPersonCharacter.BP_FirstPersonCharacter_C|GetFirstPersonCamera _asbp_first_person_character))) 1e+03)) "TraceTypeQuery1" false 0 "Persistent"))
      (Math|Integer|DecrementInt (Variables|Default|GetCurrentAmmo)
        (:%20%20
          (Game|Damage|ApplyDamage (.HitActor (Collision|BreakHitResult _outhit)) 1e+01 0 0))))))

(fn Reload)