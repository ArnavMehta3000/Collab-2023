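; BP_MasterPlayer is the first-person player character, handling movement, ladder exit, pause menu, vision mode, combat and gadgets.
; On BeginPlay it caches the gun model, run game mode and game instance, then sets up the HUD and character-specific arms.
; Gadget counts live in the game instance, gating EMP, sound and trap spawns, with events refreshing the HUD.
; Damage costs fixed health until death disables input; camera peeking logic is disconnected.
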(event Custom|InitHUD
  (if (Variables|Default|GetisInRun)
    (bind _returnvalue (UserInterface|CreateWidget "/Game/Master/Blueprint/UI/WB_PlayerHud.WB_PlayerHud_C" (Game|GetPlayerController 0)))
    (bind _output_get (Variables|Default|SetplayerHUD _returnvalue))
    (Class|IInitable|Initialize(Message) _output_get)
    (UserInterface|Viewport|AddtoPlayerScreen _output_get)
    (Default|UpdateGadgetCount _output_get) ; Read number of gadgets from instance
    (EventDispatchers|BindEventtoOnUseGadget (delegate Custom|OnUseGadget_Event))
    (EventDispatchers|BindEventtoOnPickUp (delegate Custom|OnPickUp_Event))))

(event Custom|SwordLineTrace
  (bind _meleesystem (Variables|Default|GetMeleeSystem))
  ;[0 0 0] Melee_System
  (bind _outhit (Collision|LineTraceByChannel (Transformation|GetSocketLocation _meleesystem "None") (Transformation|GetSocketLocation _meleesystem "None") "TraceTypeQuery1" false 0 "Persistent"))
  (Game|Damage|ApplyDamage (.HitActor (Collision|BreakHitResult _outhit)) 1e+01 0 0)
  (Development|PrintString "OW!"))

(event Custom|StopTriggerSword
  ;[0 0 0] Melee_System
  (Utilities|Time|ClearandInvalidateTimerbyHandle (Variables|Default|GetTriggerMeleeEvent)))

(event Custom|TriggersSword
  ;[0 0 0] Melee_System
  (bind _returnvalue (Utilities|Time|SetTimerbyEvent (delegate Custom|SwordLineTrace) 0.01))
  (Variables|Default|SetTriggerMeleeEvent _returnvalue))

(event Custom|OnPickUp_Event
  (params (gadgeType :type E_GadgetType%20Enum :default "NewEnumerator1") (isAmmoOverride :type Boolean))
  (if (Variables|Default|GetisInRun)
    (if (not isAmmoOverride)
      (Default|PickGadget (Variables|Default|GetgameInstance) gadgeType)
      (Default|UpdateGadgetCount (Variables|Default|GetplayerHUD)) ; Read number of gadgets from instance
    )))

(event Custom|OnUseGadget_Event
  (params (gadgetType :type E_GadgetType%20Enum :default "NewEnumerator1"))
  (if (Variables|Default|GetisInRun)
    (Default|UseGadget (Variables|Default|GetgameInstance) gadgetType)
    (Default|UpdateGadgetCount (Variables|Default|GetplayerHUD)) ; Read number of gadgets from instance
  ))

(event Custom|PlayerDeath
  (Input|DisableInput (Game|GetPlayerController 0)))

(event EventBeginPlay
  ;[0 0 0] Begin Play
  (Utilities|FlowControl|Delay 0.3)
  (bind _asbp_player_gun_model (Utilities|Casting|CastToBP_PlayerGunModel (Variables|/Script/Engine.ChildActorComponent|GetChildActor (Variables|Default|GetBP_PlayerGunModel))))
  (Variables|Default|SetGunModel _asbp_player_gun_model)
  (bind _asgm_run (Utilities|CaptureRunGameMode)
    (:Success
      (Variables|Default|SetrunGameMode _asgm_run)
      (Variables|Default|SetisInRun true)
      (bind _asincognito_gameinstance (Utilities|Casting|CastToIncognitoGameinstance (Game|GetGameInstance))
        (:then
          (Variables|Default|SetgameInstance _asincognito_gameinstance)
          (CallFunction|InitHUD)
          (EventDispatchers|BindEventtoOnPlayerDeath (delegate Custom|PlayerDeath) :!label _label)
          (CallFunction|UpdateModel))
        (:CastFailed
          (Development|PrintString "FAILED TO GET GAME INSTANCE"))))
    (:Fail
      (Variables|Default|SetisInRun false)
      (Development|PrintString "Not in run level (failed to cache run game mode in master player)" true true "(R=1.000000,G=0.000000,B=0.442750,A=1.000000)" 5.0)
      (goto _label))))

(event Game|Damage|EventAnyDamage
  (params (Damage :type Float%20%28single-precision%29) (DamageType :type Damage%20Type%20Object%20Reference) (InstigatedBy :type Controller%20Object%20Reference) (DamageCauser :type Actor%20Object%20Reference))
  ;[0 0 0] Health/Respawn
  (bind _output_get (Variables|Default|SetHealth (- (Variables|Default|GetHealth) 1e+01)))
  (if (<= _output_get 0.0)
    (Default|CallOnPlayerDeath)))

(event Input|ActionEvents|InputActionPeakLeft
  (params (Key :type Key%20Structure :default "None"))
  ;[0.01042 0.01042 0.01042] Input and Movement
  ;;[0 0 0] Peaking
)

(event Input|ActionEvents|InputActionPeakRight
  (params (Key :type Key%20Structure :default "None"))
  ;[0.01042 0.01042 0.01042] Input and Movement
  ;;[0 0 0] Peaking
)

(event Input|ActionEvents|InputActionShoot
  (params (Key :type Key%20Structure :default "None"))
  ;[0 0 0] Shooting
  (:Pressed
    (Utilities|FlowControl|Sequence
      (:then_0
        (Default|StartShooting (Variables|Default|GetGunModel) (Variables|Default|GetCamera)))
      (:then_1
        (Utilities|FlowControl|DoOnce false :!label _label
          (:Completed
            (Default|PlayShootMontage (Variables|Default|GetGunModel))
            (Components|Animation|PlayAnimation (Variables|Default|GetGun) "/Game/Animation/Billy/ArmRig/Animations/GunAnimations/Gun/FiringGun.FiringGun" false)
            (Animation|Montage|PlayMontage (Variables|Default|GetFPSArms) "/Game/Animation/Billy/ArmRig/Animations/GunAnimations/ArmsFire.ArmsFire"
              (:OnCompleted
                (goto _label Reset))
              (:OnInterrupted
                (goto _label Reset)))))))))

(event Input|ActionEvents|InputActionSprint
  (params (Key :type Key%20Structure :default "None"))
  (bind _charactermovement (Variables|Character|GetCharacterMovement))
  ;[0.01042 0.01042 0.01042] Input and Movement
  ;;[0 0 0] Sprinting
  (:Pressed
    (Variables|/Script/Engine.CharacterMovementComponent|SetMaxWalkSpeed _charactermovement 1.5e+03))
  (:Released
    (Variables|/Script/Engine.CharacterMovementComponent|SetMaxWalkSpeed _charactermovement 6e+02)))

(event Input|ActionEvents|InputActionCrouch
  (params (Key :type Key%20Structure :default "None"))
  ;[0.01042 0.01042 0.01042] Input and Movement
  ;;[0 0 0] Crouch
  (:Pressed
    (Character|Crouch))
  (:Released
    (Character|UnCrouch)))

(event Input|ActionEvents|InputActionJump
  (params (Key :type Key%20Structure :default "None"))
  ;[0.01042 0.01042 0.01042] Input and Movement
  ;;[0 0 0] Jumping
  (:Pressed
    (if (Class|NavMovementComponent|IsFlying (Variables|Character|GetCharacterMovement))
      (CallFunction|GetOffLadder -5e+01))
    (Character|Jump))
  (:Released
    (Character|StopJumping)))

(event Input|AxisEvents|InputAxisMoveForward/Backward
  (params (AxisValue :type Float%20%28single-precision%29))
  ;[0.01042 0.01042 0.01042] Input and Movement
  ;;[0 0 0] Movement
  (Pawn|Input|AddMovementInput (select (Class|NavMovementComponent|IsFlying (Variables|Character|GetCharacterMovement)) (Math|Vector|GetForwardVector (Variables|Default|GetCamera)) (Transformation|GetActorForwardVector)) AxisValue false))

(event Input|AxisEvents|InputAxisTurnRight/LeftMouse
  (params (AxisValue :type Float%20%28single-precision%29))
  ;[0.01042 0.01042 0.01042] Input and Movement
  ;;[0 0 0] Camera - Mouse
  (Pawn|Input|AddControllerYawInput AxisValue))

(event Input|AxisEvents|InputAxisLookUp/DownMouse
  (params (AxisValue :type Float%20%28single-precision%29))
  ;[0.01042 0.01042 0.01042] Input and Movement
  ;;[0 0 0] Camera - Mouse
  (Pawn|Input|AddControllerPitchInput AxisValue))

(event Input|AxisEvents|InputAxisMoveRight/Left
  (params (AxisValue :type Float%20%28single-precision%29))
  (bind _returnvalue (Pawn|GetControlRotation :!class /Script/Engine.Pawn))
  ;[0.01042 0.01042 0.01042] Input and Movement
  ;;[0 0 0] Movement
  (Pawn|Input|AddMovementInput (Math|Vector|GetRightVector (Math|Rotator|MakeRotator (.roll _returnvalue) 0.0 (.yaw _returnvalue))) AxisValue false))

(event Input|KeyboardEvents|Y
  (params (Key :type Key%20Structure :default "None"))
  ;[0 0 0] Test Gadget Use
  (:Pressed
    (bind _canuse (CallFunction|CanUseGadget "NewEnumerator1"))
    (if _canuse
      (CallFunction|SpawnGadget "NewEnumerator1")
      (Default|CallOnUseGadget "NewEnumerator1"))))

(event Input|KeyboardEvents|U
  (params (Key :type Key%20Structure :default "None"))
  ;[0 0 0] Test Gadget Use
  (:Pressed
    (bind _canuse (CallFunction|CanUseGadget "NewEnumerator2"))
    (if _canuse
      (CallFunction|SpawnGadget "NewEnumerator2")
      (Default|CallOnUseGadget "NewEnumerator2"))))

(event Input|MouseEvents|RightMouseButton
  (params (Key :type Key%20Structure :default "None"))
  ;[0 0 0] Melee_System
  (:Pressed
    (Utilities|FlowControl|DoOnce false :!label _label
      (:Completed
        (bind _returnvalue (Animation|PlayAnimMontage 0 1.0 "None"))
        (Utilities|FlowControl|Delay _returnvalue)
        (goto _label Reset)))))

(event Input|KeyboardEvents|B
  (params (Key :type Key%20Structure :default "None"))
  ;[0 0 0] VisionMode
  (:Pressed
    (Utilities|FlowControl|FlipFlop
      (:A
        (bind _newtrack_0 (Timeline|Timeline_1 Play)
          (:Update
            (Rendering|Material|SetScalarParameterValue "/Game/Master/Blueprint/Materials/Vision.Vision" "VisionOn" _newtrack_0 :!class /Script/Engine.KismetMaterialLibrary))))
      (:B
        (Timeline|Timeline_1 Reverse)))))

(event Input|KeyboardEvents|V
  (params (Key :type Key%20Structure :default "None"))
  (bind _knife (Variables|Default|GetKnife))
  ;[1 1 1] Reload Melee and throwing animation
  (:Pressed
    (Utilities|FlowControl|DoOnce false :!label _label
      (:Completed
        (Rendering|SetVisibility _knife true false)
        (Animation|Montage|PlayMontage (Variables|Default|GetFPSArms) "/Game/Animation/Billy/ArmRig/Animations/GunAnimations/MCKnife_Montage.MCKnife_Montage"
          (:OnBlendOut
            _)
          (:OnInterrupted
            _))
        (Rendering|SetVisibility _knife false false)
        (Utilities|FlowControl|Sequence
          (:then_0
            (goto _label Reset))
          (:then_1
            (goto _label Reset)))))))

(event Input|KeyboardEvents|I
  (params (Key :type Key%20Structure :default "None"))
  ;[0 0 0] Test Gadget Use
  (:Pressed
    (bind _canuse (CallFunction|CanUseGadget "NewEnumerator5"))
    (if _canuse
      (CallFunction|SpawnGadget "NewEnumerator5")
      (Default|CallOnUseGadget "NewEnumerator5"))))

(event Input|KeyboardEvents|R
  (params (Key :type Key%20Structure :default "None"))
  ;[1 1 1] Reload Melee and throwing animation
  (:Pressed
    (Utilities|FlowControl|DoOnce false :!label _label
      (:Completed
        (Components|Animation|PlayAnimation (Variables|Default|GetGun) "/Game/Animation/Billy/ArmRig/Animations/GunAnimations/Gun/GunReload.GunReload" false)
        (Animation|Montage|PlayMontage (Variables|Default|GetFPSArms) "/Game/Animation/Billy/ArmRig/Animations/GunAnimations/ReloadMon.ReloadMon"
          (:OnCompleted
            (goto _label Reset))
          (:OnInterrupted
            (goto _label Reset)))))))

(event Input|KeyboardEvents|Q
  (params (Key :type Key%20Structure :default "None"))
  ;[1 1 1] Reload Melee and throwing animation
  (:Pressed
    (Utilities|FlowControl|DoOnce false :!label _label
      (:Completed
        (Rendering|SetVisibility (Variables|Default|GetGrenade) true false)
        (Utilities|FlowControl|Sequence
          (:then_0
            (Animation|Montage|PlayMontage (Variables|Default|GetFPSArms) "/Game/Animation/Billy/ArmRig/Animations/GunAnimations/ThrowingAnim_Montage.ThrowingAnim_Montage"
              (:OnCompleted
                (goto _label Reset))
              (:OnInterrupted
                (goto _label Reset))))
          (:then_1
            (Utilities|FlowControl|Delay 1.5)
            (Rendering|SetVisibility (Variables|Default|GetGrenade) false false)))))))

(event Input|KeyboardEvents|Escape
  (params (Key :type Key%20Structure :default "None"))
  (bind _returnvalue (Game|GetPlayerController 0))
  (bind _returnvalue_2 (Game|GetPlayerController 0))
  ;[0 0 0] Pausing
  (:Pressed
    (Utilities|FlowControl|FlipFlop
      (:A
        (Input|SetInputModeGameandUI _returnvalue_2 0 "DoNotLock" true false)
        (bind _returnvalue_3 (UserInterface|CreateWidget "/Game/Master/Blueprint/UI/Pause_Menu.Pause_Menu_C"))
        (Variables|/Script/Engine.PlayerController|SetbShowMouseCursor _returnvalue_2 true)
        (UserInterface|Viewport|AddtoViewport _returnvalue_3 0)
        (Game|SetGamePaused true))
      (:B
        (Viewport|RemoveAllWidgets)
        (Game|SetGamePaused false)
        (Input|SetInputModeGameOnly _returnvalue false)
        (Variables|/Script/Engine.PlayerController|SetbShowMouseCursor _returnvalue false)
        (bind _returnvalue_4 (UserInterface|CreateWidget "/Game/Master/Blueprint/UI/WB_PlayerHud.WB_PlayerHud_C"))
        (UserInterface|Viewport|AddtoViewport _returnvalue_4 0)))))

(event Input|TouchEvents|InputTouch
  (params (Location :type Vector) (FingerIndex :type ETouchIndex%20Enum))
  ;[0.01042 0.01042 0.01042] Input and Movement
  ;;[0 0 0] Jumping
  (:Pressed
    (if (Class|NavMovementComponent|IsFlying (Variables|Character|GetCharacterMovement))
      (CallFunction|GetOffLadder -5e+01))
    (Character|Jump))
  (:Released
    (Character|StopJumping)))

(fn ConstructionScript
  (Variables|Default|SetCamera%20Default%20Transform (Transformation|GetRelativeTransform (Variables|Default|GetCamera))))

(fn GetOffLadder
  (params (launchForce :type Float%20%28double-precision%29))
  (bind _returnvalue (Transformation|GetActorForwardVector))
  (bind _returnvalue_2 (* _returnvalue launchForce))
  (Character|LaunchCharacter (Math|Vector|MakeVector (.x _returnvalue_2) (.y _returnvalue_2) 0.0) false false))

(fn Invisibilityon
  (Rendering|Material|SetMaterial (Variables|Character|GetMesh) 0 "/Game/Master/Blueprint/Materials/Invisibility.Invisibility")
  (return))

(fn InvisibilityOff
  (Rendering|Material|SetMaterial (Variables|Character|GetMesh) 0 "/Game/Art/Characters/FPMarms/Materials/02_-_Default.02_-_Default")
  (return))

(fn UpdateRoomRef
  (params (playerRoomRef :type BP%20New%20Room%20Base%20Object%20Reference))
  (Default|UpdatePlayerRoomRef (Variables|Default|GetrunGameMode) playerRoomRef))

(fn TryDoSoundGadget
  (bind _returnvalue (Transformation|GetActorTransform))
  (Game|SpawnActorfromClass "/Game/Tech/Chris/Blueprints/Weaponsandgadgets/BP_SoundGadget.BP_SoundGadget_C" (Math|Transform|MakeTransform (+ (* (Transformation|GetActorForwardVector) 1.5e+02) (.location _returnvalue)) (.rotation _returnvalue) (Math|Conversions|ToVector(Float) 1.0)) "AdjustIfPossibleButAlwaysSpawn" 0 0))

(fn CanUseGadget
  (params (type :type E_GadgetType%20Enum :default "NewEnumerator1"))
  (bind _gameinstance (Variables|Default|GetgameInstance))
  (bind _stats (Variables|/Game/Master/Blueprint/GameModes/IncognitoGameinstance.IncognitoGameinstance_C|Getstats _gameinstance))
  (Utilities|IsValid _gameinstance
    (:Is%20Valid
      (switch Utilities|FlowControl|Switch|SwitchonE_GadgetType type
        (:NewEnumerator1
          (if (> (.currentempgadgetcount _stats) 0)
            _
            (else
              (return false))))
        (:NewEnumerator2
          (if (> (.currentsoundgadgetcount _stats) 0)
            _
            (else
              (return false))))
        (:NewEnumerator5
          (if (> (.currenttrapgadgetcount _stats) 0)
            _
            (else
              (return false)))))
      (return true))))

(fn SpawnGadget
  (params (Gadget :type E_GadgetType%20Enum :default "NewEnumerator1"))
  (Game|SpawnActorfromClass (Utilities|Select :Index Gadget :NewEnumerator1 "/Game/Tech/Chris/Blueprints/Weaponsandgadgets/BP_EMP.BP_EMP_C" :NewEnumerator2 "/Game/Tech/Chris/Blueprints/Weaponsandgadgets/BP_SoundGadget.BP_SoundGadget_C" :NewEnumerator5 "/Game/Tech/Chris/Blueprints/Weaponsandgadgets/BP_Trap.BP_Trap_C") (Math|Transform|MakeTransform (Transformation|GetWorldLocation (Variables|Default|GetArrow1)) "0, 0, 0" "1.000000,1.000000,1.000000") "AdjustIfPossibleButAlwaysSpawn" 0 0))

(fn UpdateModel
  (Variables|/Script/Engine.SkeletalMeshComponent|SetSkeletalMeshAsset (Variables|Default|GetFPSArms) (Utilities|Select :Index (Variables|/Game/Master/Blueprint/GameModes/IncognitoGameinstance.IncognitoGameinstance_C|GetcharacterType (.AsIncognito%20Gameinstance (Utilities|Casting|CastToIncognitoGameinstance (Game|GetGameInstance)))) :NewEnumerator0 "/Game/Animation/Billy/ArmRig/MaleRig.MaleRig" :NewEnumerator1 "/Game/Animation/Billy/ArmRig/Rig.Rig")))