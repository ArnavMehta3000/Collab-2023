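; BP_HubShop is a hub shop Blueprint whose Shop component grows into view when something overlaps its Box and shrinks away when the overlap ends.
; The construction script caches Shop's world scale as OrigScale, and BeginPlay collapses Shop to zero scale.
; The Shop_scale timeline lerps between zero and OrigScale, playing on begin overlap and reversing on end overlap, with no filter on the overlapping actor.
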(event OnComponentBeginOverlap(Box)
  (params (OverlappedComponent :type Primitive%20Component%20Object%20Reference) (OtherActor :type Actor%20Object%20Reference) (OtherComp :type Primitive%20Component%20Object%20Reference) (OtherBodyIndex :type Integer) (bFromSweep :type Boolean) (SweepResult :type Hit%20Result%20Structure%20%28by%20ref%29))
  (bind _alpha (Timeline|Shop_scale Play)
    (:Update
      (Transformation|SetWorldScale3D (Variables|Default|GetShop) (Math|Vector|Lerp(Vector) "0, 0, 0" (Variables|Default|Getorig_Scale) _alpha)))))

(event OnComponentEndOverlap(Box)
  (params (OverlappedComponent :type Primitive%20Component%20Object%20Reference) (OtherActor :type Actor%20Object%20Reference) (OtherComp :type Primitive%20Component%20Object%20Reference) (OtherBodyIndex :type Integer))
  (bind _alpha (Timeline|Shop_scale Reverse)
    (:Update
      (Transformation|SetWorldScale3D (Variables|Default|GetShop) (Math|Vector|Lerp(Vector) "0, 0, 0" (Variables|Default|Getorig_Scale) _alpha)))))

(event EventBeginPlay
  (Transformation|SetWorldScale3D (Variables|Default|GetShop) "0, 0, 0"))

(fn ConstructionScript
  (Variables|Default|Setorig_Scale (Transformation|GetWorldScale (Variables|Default|GetShop))))