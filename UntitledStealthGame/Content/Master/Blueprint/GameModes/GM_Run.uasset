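; GM_Run is the game mode for a run, which starts generation on BeginPlay through the first BP_Generator found in the level.
; It stores the player's current room, announcing changes through an OnRoomUpdate call and exposing the reference via a getter.
; InRoomBounds tests whether a location lies inside that room, using min and max bounds around the room actor's location, and prints an error without a room reference.
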(event EventBeginPlay
  (bind _outactors (Actor|GetAllActorsOfClass "/Game/Tech/Arnav/Blueprints/BP_Generator.BP_Generator_C"))
  (Default|FireGeneration (Utilities|Array|Get(acopy) _outactors)))

(fn ConstructionScript)

(fn UpdatePlayerRoomRef
  (params (playerRoomRef :type BP%20New%20Room%20Base%20Object%20Reference))
  (bind _output_get (Variables|Default|SetplayerRoomRef playerRoomRef))
  (Default|CallOnRoomUpdate _output_get))

(fn GetCurrentRoom
  (return (Variables|Default|GetplayerRoomRef)))

(fn InRoomBounds
  (params (testLocation :type Vector))
  (bind _playerroomref (Variables|Default|GetplayerRoomRef))
  (bind _returnvalue (Transformation|GetActorLocation _playerroomref))
  (Utilities|IsValid _playerroomref
    (:Is%20Valid
      (bind _output_get (LocalVariables|SetmaxBounds (Utilities|GetMaxBounds _returnvalue)))
      (bind _output_get_2 (LocalVariables|SetminBounds (Utilities|GetMinBounds _returnvalue)))
      (if (and (Math|Boolean|ANDBoolean (<= (.x testLocation) (.x _output_get)) (<= (.y testLocation) (.y _output_get)) (<= (.z testLocation) (.z _output_get))) (Math|Boolean|ANDBoolean (>= (.x testLocation) (.x _output_get_2)) (>= (.y testLocation) (.y _output_get_2)) (>= (.z testLocation) (.z _output_get_2))))
        (return true)
        (else
          (return false))))
    (:Is%20Not%20Valid
      (Development|PrintString "GM_RUN: NO ROOM REF!!!!!!!!!!!!!!!!!!!!!!!!!" true true "(R=1.000000,G=0.000000,B=0.666844,A=1.000000)" 1e+01))))

(fn SetRoomHalfSize
  (params (roomHalfSize :type Float%20%28double-precision%29))
  (Variables|Default|SetroomHalfSize roomHalfSize))