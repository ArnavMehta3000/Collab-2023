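; Game instance for Incognito that holds player points, shop costs and EMP, sound and trap gadget counts.
; Init seeds starting points, the cost struct and gadget maximums, with functions to add or subtract points and read costs.
; UseGadget and PickGadget step the matching current count in the Stats struct without limit checks.
; SetCountByCost derives counts from costs through CostToCount, whose division-and-add formula is left unconnected.
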(event EventInit
  (Variables|Default|SetplayerPoints 100) ; Set player starting points
  (|SetBy-RefVar (Variables|Default|GetmaxCosts) (Utilities|Struct|MakeS_Costs (Variables|Defaults|GetroomBonus) (Variables|Defaults|GetempCost) (Variables|Defaults|GetsoundCost) (Variables|Defaults|GettrapCost) (Variables|Defaults|GetammoCost)))
  (|SetBy-RefVar (Variables|Default|Getstats) (Utilities|Struct|MakeS_GadgetStats (Variables|Defaults|GetmaxSound) (Variables|Defaults|GetmaxEmp) (Variables|Defaults|GetmaxTrap) 0 0 0)))

(fn AddPlayerPoints
  (params (toAdd :type Integer))
  (Variables|Default|SetplayerPoints (+ toAdd (Variables|Default|GetplayerPoints))))

(fn GetCosts
  (bind _maxcosts (Variables|Default|GetmaxCosts))
  (return (.clearroombonus _maxcosts) (.empgadgetcost _maxcosts) (.soundgadgetcost _maxcosts) (.trapgadgetcost _maxcosts) (.ammocost _maxcosts)))

(fn SetCountbyCost
  (params (soundCost :type Integer) (empCost :type Integer) (trapCost :type Integer))
  (bind _stats (Variables|Default|Getstats))
  (bind (_maxsoundgadgetcount _maxempgadgetcount _maxtrapgadgetcount _currentsoundgadgetcount _currentempgadgetcount _currenttrapgadgetcount) (Utilities|Struct|BreakS_GadgetStats _stats))
  (|SetBy-RefVar _stats (Utilities|Struct|MakeS_GadgetStats (Variables|Defaults|GetmaxSound) (Variables|Defaults|GetmaxEmp) (Variables|Defaults|GetmaxTrap) (Utilities|CosttoCount soundCost (Variables|Defaults|GetsoundCost) _currentsoundgadgetcount) (Utilities|CosttoCount empCost (Variables|Defaults|GetempCost) _currentempgadgetcount) (Utilities|CosttoCount trapCost (Variables|Defaults|GettrapCost) _currenttrapgadgetcount))))

(fn SubtractPlayerPoints
  (params (toRemove :type Integer))
  (Variables|Default|SetplayerPoints (- (Variables|Default|GetplayerPoints) toRemove)))

(fn UseGadget
  (params (gadget :type E_GadgetType%20Enum :default "NewEnumerator1"))
  (bind _stats (Variables|Default|Getstats))
  (bind (_maxsoundgadgetcount _maxempgadgetcount _maxtrapgadgetcount _currentsoundgadgetcount _currentempgadgetcount _currenttrapgadgetcount) (Utilities|Struct|BreakS_GadgetStats _stats))
  (switch Utilities|FlowControl|Switch|SwitchonE_GadgetType gadget
    (:NewEnumerator1
      (|SetBy-RefVar _stats (Utilities|Struct|MakeS_GadgetStats _maxsoundgadgetcount _maxempgadgetcount _maxtrapgadgetcount _currentsoundgadgetcount (- _currentempgadgetcount 1) _currenttrapgadgetcount)))
    (:NewEnumerator2
      (|SetBy-RefVar _stats (Utilities|Struct|MakeS_GadgetStats _maxsoundgadgetcount _maxempgadgetcount _maxtrapgadgetcount (- _currentsoundgadgetcount 1) _currentempgadgetcount _currenttrapgadgetcount)))
    (:NewEnumerator5
      (|SetBy-RefVar _stats (Utilities|Struct|MakeS_GadgetStats _maxsoundgadgetcount _maxempgadgetcount _maxtrapgadgetcount _currentsoundgadgetcount _currentempgadgetcount (- _currenttrapgadgetcount 1))))))

(fn PickGadget
  (params (gadget :type E_GadgetType%20Enum :default "NewEnumerator1"))
  (bind _stats (Variables|Default|Getstats))
  (bind (_maxsoundgadgetcount _maxempgadgetcount _maxtrapgadgetcount _currentsoundgadgetcount _currentempgadgetcount _currenttrapgadgetcount) (Utilities|Struct|BreakS_GadgetStats _stats))
  (switch Utilities|FlowControl|Switch|SwitchonE_GadgetType gadget
    (:NewEnumerator1
      (|SetBy-RefVar _stats (Utilities|Struct|MakeS_GadgetStats _maxsoundgadgetcount _maxempgadgetcount _maxtrapgadgetcount _currentsoundgadgetcount (+ _currentempgadgetcount 1) _currenttrapgadgetcount)))
    (:NewEnumerator2
      (|SetBy-RefVar _stats (Utilities|Struct|MakeS_GadgetStats _maxsoundgadgetcount _maxempgadgetcount _maxtrapgadgetcount (+ _currentsoundgadgetcount 1) _currentempgadgetcount _currenttrapgadgetcount)))
    (:NewEnumerator5
      (|SetBy-RefVar _stats (Utilities|Struct|MakeS_GadgetStats _maxsoundgadgetcount _maxempgadgetcount _maxtrapgadgetcount _currentsoundgadgetcount _currentempgadgetcount (+ _currenttrapgadgetcount 1))))))