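; Main menu game mode that initializes the menu player controller, main menu widget and options suitcase actor.
; Three level sequences drive the view: looping menu and options shots, joined by a double-speed transition played forward or in reverse.
; Resettable DoOnce gates on the transition's finished callback start the next loop, re-adding the menu widget on return.
; Play opens the hub level with a loading screen and requests game-only input after a delay.
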(event Custom|CreateSequences
  ;[0 0 0] Create Sequences
  (bind _returnvalue (Sequencer|Player|CreateLevelSequencePlayer "/Game/Cinematics/Sequences/TrainMenu/TrainMenuMaster.TrainMenuMaster"))
  (Variables|Sequences|Setcam1Sequence _returnvalue)
  (bind _returnvalue_2 (Sequencer|Player|CreateLevelSequencePlayer "/Game/Cinematics/Sequences/TrainOptions/TrainOptionsMaster.TrainOptionsMaster" (Utilities|Struct|MakeMovieSceneSequencePlaybackSettings false (Utilities|Struct|MakeMovieSceneSequenceLoopCount 0) 2.0 0.0 false false false false false false false false)))
  (Variables|Sequences|Setcam2Sequence _returnvalue_2)
  (bind _returnvalue_3 (Sequencer|Player|CreateLevelSequencePlayer "/Game/Cinematics/Sequences/TrainOptionsStay/TrainOptionsStayMaster.TrainOptionsStayMaster"))
  (Variables|Sequences|Setcam3Sequence _returnvalue_3))

(event Custom|OnPlayGame
  (bind _returnvalue (Game|GetPlayerController 0))
  ;[0 0 0] Go To Hub (PLAY GAME)
  (Audio|PlaySound2D "/Engine/VREditor/Sounds/UI/Click_on_Button_Cue.Click_on_Button_Cue" 1.0 1.0 0.0 0 0)
  (Game|OpenLevel(byObjectReference) "/Game/Master/Hub/HubLevels/L_Hub_Structure.L_Hub_Structure")
  (bind _returnvalue_2 (UserInterface|CreateWidget "/Game/Master/Blueprint/UI/LoadingScreen.LoadingScreen_C" _returnvalue))
  (UserInterface|Viewport|AddtoViewport _returnvalue_2 0)
  (Utilities|FlowControl|Delay 3.0)
  (Widget|RemovefromParent (Variables|Default|GetLoading_screen))
  (Input|SetInputModeGameOnly _returnvalue false))

(event Custom|OnShowOptions
  (bind _cam2sequence (Variables|Sequences|Getcam2Sequence))
  ;[0 0 0] Show Options Suitcase
  (Utilities|FlowControl|Sequence
    (:then_0
      (Widget|RemovefromParent (Variables|Default|GetmenuWidget))
      (Utilities|FlowControl|DoOnce false) ; enters at Reset
    )
    (:then_1
      (Class|MovieSceneSequencePlayer|StopatCurrentTime (Variables|Sequences|Getcam1Sequence))
      (Sequencer|Player|Play _cam2sequence :!class /Script/MovieScene.MovieSceneSequencePlayer)
      (EventDispatchers|AssignOnFinished _cam2sequence (delegate Custom|OnFinished_Event)))))

(event Custom|OnFinished_Event
  ;[0 0 0] Show Options Suitcase
  (Utilities|FlowControl|DoOnce false
    (:Completed
      (Class|MovieSceneSequencePlayer|PlayLooping (Variables|Sequences|Getcam3Sequence) -1))))

(event Custom|CreateMenuUI
  (bind _returnvalue (UserInterface|CreateWidget "/Game/Master/Blueprint/UI/WB_MainMenu.WB_MainMenu_C"))
  (bind _output_get (Variables|Default|SetmenuWidget _returnvalue))
  (Class|IInitable|Initialize(Message) _output_get)
  (bind _outactors (Actor|GetAllActorsOfClass "/Game/Master/Blueprint/BP_OptionsSuitcase.BP_OptionsSuitcase_C"))
  (bind _output_get_2 (Variables|Default|SetoptionsSuitcase (Utilities|Array|Get(acopy) _outactors)))
  (Class|IInitable|Initialize(Message) _output_get_2))

(event Custom|GoBackToMainMenu
  (bind _cam2sequence (Variables|Sequences|Getcam2Sequence))
  ;[0 0 0] Go Back To Main Menu (from options)
  (Utilities|FlowControl|Sequence
    (:then_0
      (Utilities|FlowControl|DoOnce false) ; enters at Reset
    )
    (:then_1
      (Class|MovieSceneSequencePlayer|StopatCurrentTime (Variables|Sequences|Getcam3Sequence))
      (Class|MovieSceneSequencePlayer|PlayReverse _cam2sequence)
      (EventDispatchers|AssignOnFinished _cam2sequence (delegate Custom|OnFinished_Event_0)))))

(event Custom|OnFinished_Event_0
  ;[0 0 0] Go Back To Main Menu (from options)
  (Utilities|FlowControl|DoOnce false
    (:Completed
      (Class|MovieSceneSequencePlayer|PlayLooping (Variables|Sequences|Getcam1Sequence) -1)
      (UserInterface|Viewport|AddtoViewport (Variables|Default|GetmenuWidget) 0))))

(event EventBeginPlay
  (Utilities|FlowControl|Sequence
    (:then_0
      (bind _asbp_menu_player (Utilities|Casting|CastToBP_MenuPlayer (Game|GetPlayerController 0)))
      (bind _output_get (Variables|Default|SetmenuPlayerController _asbp_menu_player))
      (Class|IInitable|Initialize(Message) _output_get))
    (:then_1
      (CallFunction|CreateSequences))
    (:then_2
      (CallFunction|CreateMenuUI)
      (UserInterface|Viewport|AddtoViewport (Variables|Default|GetmenuWidget) 0)
      (Class|MovieSceneSequencePlayer|PlayLooping (Variables|Sequences|Getcam1Sequence) -1))))

(fn ConstructionScript)