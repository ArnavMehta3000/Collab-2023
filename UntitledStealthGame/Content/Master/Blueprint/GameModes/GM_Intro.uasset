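; GM_Intro is the game mode that plays the intro video, then moves on to the main menu.
; On BeginPlay it creates a WB_IntroPlayer widget for the first player controller, adds it to the viewport, starts playback and binds to its OnFinished event.
; When that fires, it removes all widgets and opens L_MainMenu.
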(event Custom|OnFinished_Event
  (Viewport|RemoveAllWidgets)
  (Game|OpenLevel(byObjectReference) "/Game/Master/MainMenu/L_MainMenu.L_MainMenu"))

(event EventBeginPlay
  (bind _returnvalue (Game|GetPlayerController 0))
  (Development|PrintString (Utilities|GetDisplayName _returnvalue))
  (bind _returnvalue_2 (UserInterface|CreateWidget "/Game/Master/Blueprint/UI/WB_IntroPlayer.WB_IntroPlayer_C" _returnvalue))
  (bind _output_get (Variables|Default|SetintroVideo _returnvalue_2))
  (UserInterface|Viewport|AddtoViewport _output_get 0)
  (Default|PlayIntro _output_get)
  (EventDispatchers|AssignOnFinished _output_get (delegate Custom|OnFinished_Event)))

(fn ConstructionScript)