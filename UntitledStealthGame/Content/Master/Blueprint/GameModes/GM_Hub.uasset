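; Game mode for the hub level, which sets up its sublevels, player HUD and gadget shop.
; BeginPlay streams in lighting and prop level instances, then after a short delay creates both widgets and shows the HUD.
; A nonzero RUN option passes the game instance's next run generation count to the level switcher.
; Shop open and close functions toggle cursor and input mode, with closing refreshing the HUD's gadget count.
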(event Custom|CheckOptions
  (if (not (== (Class|GameplayStatics|GetIntOption (Variables|Default|GetOptionsString) "RUN") 0))
    (bind _returnvalue (Actor|GetActorOfClass "/Game/Master/Blueprint/BP_LevelSwitcher.BP_LevelSwitcher_C"))
    (Default|SetGenCount _returnvalue (Default|GetNextRunGenCount (.AsIncognito%20Gameinstance (Utilities|Casting|CastToIncognitoGameinstance (Game|GetGameInstance)))))))

(event EventBeginPlay
  (bind _returnvalue (Game|GetPlayerController 0))
  (Utilities|LoadSubLevels)
  (Utilities|FlowControl|Delay 0.25)
  (bind _returnvalue_2 (UserInterface|CreateWidget "/Game/Master/Blueprint/UI/WB_GadgetShop.WB_GadgetShop_C" _returnvalue))
  (bind _output_get (Variables|Default|SetshopWidget _returnvalue_2))
  (Class|IInitable|Initialize(Message) _output_get)
  (bind _returnvalue_3 (UserInterface|CreateWidget "/Game/Master/Blueprint/UI/WB_PlayerHud.WB_PlayerHud_C" _returnvalue))
  (bind _output_get_2 (Variables|Default|SethudWidget _returnvalue_3))
  (Class|IInitable|Initialize(Message) _output_get_2)
  (Default|UpdateGadgetCount _output_get_2)
  (UserInterface|Viewport|AddtoPlayerScreen _output_get_2)
  (CallFunction|CheckOptions))

(fn ConstructionScript)

(fn OpenShop
  (bind _returnvalue (Game|GetPlayerController 0))
  (bind _shopwidget (Variables|Default|GetshopWidget))
  (Variables|/Script/Engine.PlayerController|SetbShowMouseCursor _returnvalue true)
  (Input|SetInputModeUIOnly _returnvalue _shopwidget "DoNotLock" true)
  (Default|OpenShop _shopwidget)
  (UserInterface|Viewport|AddtoPlayerScreen _shopwidget))

(fn CloseShop
  (bind _returnvalue (Game|GetPlayerController 0))
  (bind _shopwidget (Variables|Default|GetshopWidget))
  (Input|SetInputModeGameOnly _returnvalue false)
  (Variables|/Script/Engine.PlayerController|SetbShowMouseCursor _returnvalue false)
  (Widget|RemovefromParent _shopwidget)
  (Default|ResetShop _shopwidget)
  (Default|UpdateGadgetCount (Variables|Default|GethudWidget)))