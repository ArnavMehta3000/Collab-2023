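; BP_Guvvy_Start_C1 appears to be a starting level piece that supplies spawn points for AI enemies, gadgets and keys, plus a climbable ladder.
; Initialize passes each of its placed spawn point components to the matching conversion call: ToAiSpawnPoint, ToGadgetSpawnPoint or ToKeySpawnPoint.
; Ladder begin and end overlaps forward the other actor to OnTryStartClimb and OnTryStopClimb.
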(event OnComponentBeginOverlap(Ladder)
  (params (OverlappedComponent :type Primitive%20Component%20Object%20Reference) (OtherActor :type Actor%20Object%20Reference) (OtherComp :type Primitive%20Component%20Object%20Reference) (OtherBodyIndex :type Integer) (bFromSweep :type Boolean) (SweepResult :type Hit%20Result%20Structure%20%28by%20ref%29))
  (CallFunction|OnTryStartClimb OtherActor))

(event OnComponentEndOverlap(Ladder)
  (params (OverlappedComponent :type Primitive%20Component%20Object%20Reference) (OtherActor :type Actor%20Object%20Reference) (OtherComp :type Primitive%20Component%20Object%20Reference) (OtherBodyIndex :type Integer))
  (CallFunction|OnTryStopClimb OtherActor))

(event Custom|InitAISpawns
  (CallFunction|ToAiSpawnPoint (Variables|Default|GetEnemySpawnPoint3))
  (CallFunction|ToAiSpawnPoint (Variables|Default|GetEnemySpawnPoint1))
  (CallFunction|ToAiSpawnPoint (Variables|Default|GetEnemySpawnPoint2))
  (CallFunction|ToAiSpawnPoint (Variables|Default|GetEnemySpawnPoint4))
  (CallFunction|ToAiSpawnPoint (Variables|Default|GetEnemySpawnPoint6))
  (CallFunction|ToAiSpawnPoint (Variables|Default|GetEnemySpawnPoint5))
  (CallFunction|ToAiSpawnPoint (Variables|Default|GetEnemySpawnPoint7))
  (CallFunction|ToAiSpawnPoint (Variables|Default|GetEnemySpawnPoint8))
  (CallFunction|ToAiSpawnPoint (Variables|Default|GetEnemySpawnPoint9))
  (CallFunction|ToAiSpawnPoint (Variables|Default|GetEnemySpawnPoint10))
  (CallFunction|ToAiSpawnPoint (Variables|Default|GetEnemySpawnPoint11))
  (CallFunction|ToAiSpawnPoint (Variables|Default|GetEnemySpawnPoint12))
  (CallFunction|ToAiSpawnPoint (Variables|Default|GetEnemySpawnPoint)))

(event Custom|InitGadgetSpawns
  (CallFunction|ToGadgetSpawnPoint (Variables|Default|GetGadgetSpawnPoint))
  (CallFunction|ToGadgetSpawnPoint (Variables|Default|GetGadgetSpawnPoint3))
  (CallFunction|ToGadgetSpawnPoint (Variables|Default|GetGadgetSpawnPoint2))
  (CallFunction|ToGadgetSpawnPoint (Variables|Default|GetGadgetSpawnPoint1))
  (CallFunction|ToGadgetSpawnPoint (Variables|Default|GetGadgetSpawnPoint4)))

(event Custom|InitKeySpawn
  (CallFunction|ToKeySpawnPoint (Variables|Default|GetKeySpawnLocation))
  (CallFunction|ToKeySpawnPoint (Variables|Default|GetKeySpawnLocation1))
  (CallFunction|ToKeySpawnPoint (Variables|Default|GetKeySpawnLocation2)))

(event EventBeginPlay)

(event Collision|EventActorBeginOverlap
  (params (OtherActor :type Actor%20Object%20Reference)))

(event EventTick
  (params (DeltaSeconds :type Float%20%28single-precision%29)))

(event EventInitialize
  (CallFunction|InitAISpawns)
  (CallFunction|InitGadgetSpawns)
  (CallFunction|InitKeySpawn))

(fn ConstructionScript)