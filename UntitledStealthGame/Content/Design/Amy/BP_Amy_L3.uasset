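; BP_Amy_L3 is a level layout Blueprint that sets up spawn points for AI, gadgets and keys.
; Initialize runs the gadget, key and AI setup events, each passing its hand-placed spawn references to a matching conversion helper.
; The construction script gathers all BP_AiSpawnPoint actors but leaves the result unused, as the nodes that would set enemy type and fill AiSpawnPoints are disconnected.
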(event Custom|InitGadgetSpawns
  (CallFunction|ToGadgetSpawnPoint (Variables|Default|GetGadgetSpawn))
  (CallFunction|ToGadgetSpawnPoint (Variables|Default|GetGadgetSpawn1))
  (CallFunction|ToGadgetSpawnPoint (Variables|Default|GetGadgetSpawn2))
  (CallFunction|ToGadgetSpawnPoint (Variables|Default|GetGadgetSpawn3))
  (CallFunction|ToGadgetSpawnPoint (Variables|Default|GetGadgetSpawn4))
  (CallFunction|ToGadgetSpawnPoint (Variables|Default|GetGadgetSpawn5)))

(event Custom|InitKeySpawns
  (CallFunction|ToKeySpawnPoint (Variables|Default|GetKeySpawn))
  (CallFunction|ToKeySpawnPoint (Variables|Default|GetKeySpawn1))
  (CallFunction|ToKeySpawnPoint (Variables|Default|GetKeySpawn2)))

(event Custom|InitAISpawns
  (CallFunction|ToAiSpawnPoint (Variables|Default|GetSpawn%20Point))
  (CallFunction|ToAiSpawnPoint (Variables|Default|GetSpawn%20Point1))
  (CallFunction|ToAiSpawnPoint (Variables|Default|GetSpawn%20Point2))
  (CallFunction|ToAiSpawnPoint (Variables|Default|GetSpawn%20Point3))
  (CallFunction|ToAiSpawnPoint (Variables|Default|GetSpawn%20Point4))
  (CallFunction|ToAiSpawnPoint (Variables|Default|GetSpawn%20Point5))
  (CallFunction|ToAiSpawnPoint (Variables|Default|GetSpawn%20Point6))
  (CallFunction|ToAiSpawnPoint (Variables|Default|GetSpawn%20Point7))
  (CallFunction|ToAiSpawnPoint (Variables|Default|GetSpawn%20Point8))
  (CallFunction|ToAiSpawnPoint (Variables|Default|GetSpawn%20Point9))
  (CallFunction|ToAiSpawnPoint (Variables|Default|GetSpawn%20Point10))
  (CallFunction|ToAiSpawnPoint (Variables|Default|GetSpawn%20Point11))
  (CallFunction|ToAiSpawnPoint (Variables|Default|GetSpawn%20Point12))
  (CallFunction|ToAiSpawnPoint (Variables|Default|GetSpawn%20Point13))
  (CallFunction|ToAiSpawnPoint (Variables|Default|GetSpawn%20Point14))
  (CallFunction|ToAiSpawnPoint (Variables|Default|GetSpawn%20Point15)))

(event EventInitialize
  (CallFunction|InitGadgetSpawns)
  (CallFunction|InitKeySpawns)
  (CallFunction|InitAISpawns))

(fn ConstructionScript
  (bind _outactors (Actor|GetAllActorsOfClass "/Game/Tech/Arnav/Blueprints/BP_AiSpawnPoint.BP_AiSpawnPoint_C")))