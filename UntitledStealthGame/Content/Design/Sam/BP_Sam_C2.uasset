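; BP_Sam_C2 is a child Blueprint, apparently a level piece, that provides ladders and spawn points for enemies, gadgets and keys.
; Overlaps on its four ladder components call OnTryStartClimb and OnTryStopClimb with the overlapping actor.
; Initialize runs three events that pass each placed spawn-point component to the matching AI, gadget or key conversion function.
; The construction script only calls the parent's.
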(event OnComponentBeginOverlap(Ladder)
  (params (OverlappedComponent :type Primitive%20Component%20Object%20Reference) (OtherActor :type Actor%20Object%20Reference) (OtherComp :type Primitive%20Component%20Object%20Reference) (OtherBodyIndex :type Integer) (bFromSweep :type Boolean) (SweepResult :type Hit%20Result%20Structure%20%28by%20ref%29))
  (CallFunction|OnTryStartClimb OtherActor))

(event OnComponentEndOverlap(Ladder)
  (params (OverlappedComponent :type Primitive%20Component%20Object%20Reference) (OtherActor :type Actor%20Object%20Reference) (OtherComp :type Primitive%20Component%20Object%20Reference) (OtherBodyIndex :type Integer))
  (CallFunction|OnTryStopClimb OtherActor))

(event OnComponentBeginOverlap(Ladder2)
  (params (OverlappedComponent :type Primitive%20Component%20Object%20Reference) (OtherActor :type Actor%20Object%20Reference) (OtherComp :type Primitive%20Component%20Object%20Reference) (OtherBodyIndex :type Integer) (bFromSweep :type Boolean) (SweepResult :type Hit%20Result%20Structure%20%28by%20ref%29))
  (CallFunction|OnTryStartClimb OtherActor))

(event OnComponentEndOverlap(Ladder2)
  (params (OverlappedComponent :type Primitive%20Component%20Object%20Reference) (OtherActor :type Actor%20Object%20Reference) (OtherComp :type Primitive%20Component%20Object%20Reference) (OtherBodyIndex :type Integer))
  (CallFunction|OnTryStopClimb OtherActor))

(event OnComponentBeginOverlap(Ladder3)
  (params (OverlappedComponent :type Primitive%20Component%20Object%20Reference) (OtherActor :type Actor%20Object%20Reference) (OtherComp :type Primitive%20Component%20Object%20Reference) (OtherBodyIndex :type Integer) (bFromSweep :type Boolean) (SweepResult :type Hit%20Result%20Structure%20%28by%20ref%29))
  (CallFunction|OnTryStartClimb OtherActor))

(event OnComponentEndOverlap(Ladder3)
  (params (OverlappedComponent :type Primitive%20Component%20Object%20Reference) (OtherActor :type Actor%20Object%20Reference) (OtherComp :type Primitive%20Component%20Object%20Reference) (OtherBodyIndex :type Integer))
  (CallFunction|OnTryStopClimb OtherActor))

(event OnComponentBeginOverlap(Ladder4)
  (params (OverlappedComponent :type Primitive%20Component%20Object%20Reference) (OtherActor :type Actor%20Object%20Reference) (OtherComp :type Primitive%20Component%20Object%20Reference) (OtherBodyIndex :type Integer) (bFromSweep :type Boolean) (SweepResult :type Hit%20Result%20Structure%20%28by%20ref%29))
  (CallFunction|OnTryStartClimb OtherActor))

(event OnComponentEndOverlap(Ladder4)
  (params (OverlappedComponent :type Primitive%20Component%20Object%20Reference) (OtherActor :type Actor%20Object%20Reference) (OtherComp :type Primitive%20Component%20Object%20Reference) (OtherBodyIndex :type Integer))
  (CallFunction|OnTryStopClimb OtherActor))

(event Custom|InitAiSpawns
  (CallFunction|ToAiSpawnPoint (Variables|Default|GetEnemySpawnPoint))
  (CallFunction|ToAiSpawnPoint (Variables|Default|GetEnemySpawnPoint1))
  (CallFunction|ToAiSpawnPoint (Variables|Default|GetEnemySpawnPoint2))
  (CallFunction|ToAiSpawnPoint (Variables|Default|GetEnemySpawnPoint3))
  (CallFunction|ToAiSpawnPoint (Variables|Default|GetEnemySpawnPoint4))
  (CallFunction|ToAiSpawnPoint (Variables|Default|GetEnemySpawnPoint5))
  (CallFunction|ToAiSpawnPoint (Variables|Default|GetEnemySpawnPoint6))
  (CallFunction|ToAiSpawnPoint (Variables|Default|GetEnemySpawnPoint7))
  (CallFunction|ToAiSpawnPoint (Variables|Default|GetEnemySpawnPoint8)))

(event Custom|InitKeySpawns
  (CallFunction|ToKeySpawnPoint (Variables|Default|GetKeySpawnPoint))
  (CallFunction|ToKeySpawnPoint (Variables|Default|GetKeySpawnPoint1))
  (CallFunction|ToKeySpawnPoint (Variables|Default|GetKeySpawnPoint2)))

(event Custom|InitGadgetSpawns
  (CallFunction|ToGadgetSpawnPoint (Variables|Default|GetGadgetSpawnPoint))
  (CallFunction|ToGadgetSpawnPoint (Variables|Default|GetGadgetSpawnPoint1))
  (CallFunction|ToGadgetSpawnPoint (Variables|Default|GetGadgetSpawnPoint2))
  (CallFunction|ToGadgetSpawnPoint (Variables|Default|GetGadgetSpawnPoint3))
  (CallFunction|ToGadgetSpawnPoint (Variables|Default|GetGadgetSpawnPoint4)))

(event EventInitialize
  (CallFunction|InitAiSpawns)
  (CallFunction|InitGadgetSpawns)
  (CallFunction|InitKeySpawns))

(fn ConstructionScript
  (|CallParentFunction))