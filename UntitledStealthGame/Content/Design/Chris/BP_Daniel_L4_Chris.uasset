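; Level setup Blueprint, apparently for an L4 layout, that registers spawn points for AI, gadgets and keys.
; Initialize runs three init events in sequence, one per spawn category.
; Each event makes a fixed chain of repeated conversion calls to its spawn-point type, with no arguments or further logic shown.
; The construction script is empty.
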(event Custom|InitAiSpawn
  (CallFunction|ToAiSpawnPoint)
  (CallFunction|ToAiSpawnPoint)
  (CallFunction|ToAiSpawnPoint)
  (CallFunction|ToAiSpawnPoint)
  (CallFunction|ToAiSpawnPoint)
  (CallFunction|ToAiSpawnPoint)
  (CallFunction|ToAiSpawnPoint)
  (CallFunction|ToAiSpawnPoint)
  (CallFunction|ToAiSpawnPoint)
  (CallFunction|ToAiSpawnPoint)
  (CallFunction|ToAiSpawnPoint)
  (CallFunction|ToAiSpawnPoint)
  (CallFunction|ToAiSpawnPoint)
  (CallFunction|ToAiSpawnPoint)
  (CallFunction|ToAiSpawnPoint))

(event Custom|InitGadgetSpawn
  (CallFunction|ToGadgetSpawnPoint)
  (CallFunction|ToGadgetSpawnPoint)
  (CallFunction|ToGadgetSpawnPoint)
  (CallFunction|ToGadgetSpawnPoint)
  (CallFunction|ToGadgetSpawnPoint)
  (CallFunction|ToGadgetSpawnPoint)
  (CallFunction|ToGadgetSpawnPoint))

(event Custom|InitKeySpawn
  (CallFunction|ToKeySpawnPoint)
  (CallFunction|ToKeySpawnPoint)
  (CallFunction|ToKeySpawnPoint))

(event EventInitialize
  (CallFunction|InitAiSpawn)
  (CallFunction|InitGadgetSpawn)
  (CallFunction|InitKeySpawn))

(fn ConstructionScript)