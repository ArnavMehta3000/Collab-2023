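; BP_Chris_L4 is a designer-authored layout Blueprint that declares where AI enemies, gadgets and keys can spawn.
; Its Initialize event runs three init events, one per spawn category.
; Each passes its named placement references to a matching conversion call (ToAiSpawnPoint, ToGadgetSpawnPoint or ToKeySpawnPoint), whose logic is defined outside this graph.
; The construction script only calls the parent, and BeginPlay, overlap and Tick are unused.
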(event Custom|InitAiSpawns
  (CallFunction|ToAiSpawnPoint (Variables|Default|GetEnemySpawn))
  (CallFunction|ToAiSpawnPoint (Variables|Default|GetEnemySpawn1))
  (CallFunction|ToAiSpawnPoint (Variables|Default|GetEnemySpawn2))
  (CallFunction|ToAiSpawnPoint (Variables|Default|GetEnemySpawn3))
  (CallFunction|ToAiSpawnPoint (Variables|Default|GetEnemySpawn4))
  (CallFunction|ToAiSpawnPoint (Variables|Default|GetEnemySpawn5))
  (CallFunction|ToAiSpawnPoint (Variables|Default|GetEnemySpawn6))
  (CallFunction|ToAiSpawnPoint (Variables|Default|GetEnemySpawn7))
  (CallFunction|ToAiSpawnPoint (Variables|Default|GetEnemySpawn8)))

(event Custom|InitKeySpawns
  (CallFunction|ToKeySpawnPoint (Variables|Default|GetKeySpawn))
  (CallFunction|ToKeySpawnPoint (Variables|Default|GetKeySpawn1))
  (CallFunction|ToKeySpawnPoint (Variables|Default|GetKeySpawn2)))

(event Custom|InitGadgetSpawns
  (CallFunction|ToGadgetSpawnPoint (Variables|Default|GetGadgetSpawn1))
  (CallFunction|ToGadgetSpawnPoint (Variables|Default|GetGadgetSpawn2))
  (CallFunction|ToGadgetSpawnPoint (Variables|Default|GetGadgetSpawn3))
  (CallFunction|ToGadgetSpawnPoint (Variables|Default|GetGadgetSpawn4)))

(event EventBeginPlay)

(event Collision|EventActorBeginOverlap
  (params (OtherActor :type Actor%20Object%20Reference)))

(event EventTick
  (params (DeltaSeconds :type Float%20%28single-precision%29)))

(event EventInitialize
  (CallFunction|InitAiSpawns)
  (CallFunction|InitGadgetSpawns)
  (CallFunction|InitKeySpawns))

(fn ConstructionScript
  (|CallParentFunction))