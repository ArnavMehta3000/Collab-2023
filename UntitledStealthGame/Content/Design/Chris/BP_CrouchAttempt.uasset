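; Player character Blueprint, apparently a crouch experiment, handling mouse and gamepad look, movement, touch or button jump, hold-to-crouch and left/right peeking.
; Flying mode stands in for ladder climbing: forward input follows the camera, and jumping first launches the character backward through GetOffLadder.
; Peeking plays and reverses timelines that lerp FollowCamera from the transform cached at construction toward left or right peek transforms.
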(event Input|ActionEvents|InputActionPeakLeft
  (params (Key :type Key%20Structure :default "None"))
  (bind _returnvalue (not false))
  ;[0 0 0] Peaking
  (:Pressed
    (if _returnvalue
      (bind _camera (Timeline|PeakLeft Play)
        (:Update
          (Transformation|SetRelativeTransform (Variables|Camera|GetFollowCamera) (Math|Transform|Lerp(Transform) (Variables|Default|GetcameraDefaultTransform) (Variables|Default|GetcameraPeakLeftTransform) _camera) false false)))))
  (:Released
    (if _returnvalue
      (Timeline|PeakLeft Reverse))))

(event Input|ActionEvents|InputActionPeakRight
  (params (Key :type Key%20Structure :default "None"))
  (bind _returnvalue (not false))
  ;[0 0 0] Peaking
  (:Pressed
    (if _returnvalue
      (bind _camera (Timeline|PeakRight Play)
        (:Update
          (Transformation|SetRelativeTransform (Variables|Camera|GetFollowCamera) (Math|Transform|Lerp(Transform) (Variables|Default|GetcameraDefaultTransform) (Variables|Default|GetcameraPeakRightTransform) _camera) false false)))))
  (:Released
    (if _returnvalue
      (Timeline|PeakRight Reverse))))

(event Input|ActionEvents|InputActionJump
  (params (Key :type Key%20Structure :default "None"))
  ;[0.05098 0.05098 0.05098] Jumping
  (:Pressed
    (if (Class|NavMovementComponent|IsFlying (Variables|Character|GetCharacterMovement))
      (CallFunction|GetOffLadder -5e+01))
    (Character|Jump))
  (:Released
    (Character|StopJumping)))

(event Input|AxisEvents|InputAxisMoveForward/Backward
  (params (AxisValue :type Float%20%28single-precision%29))
  ;[0.05098 0.05098 0.05098] Movement
  (Pawn|Input|AddMovementInput (select (Class|NavMovementComponent|IsFlying (Variables|Character|GetCharacterMovement)) (Math|Vector|GetForwardVector (Variables|Camera|GetFollowCamera)) (Transformation|GetActorForwardVector)) AxisValue false))

(event Input|AxisEvents|InputAxisTurnRight/LeftGamepad
  (params (AxisValue :type Float%20%28single-precision%29))
  ;[0.05098 0.05098 0.05098] Camera - Gamepad
  (Pawn|Input|AddControllerYawInput (* AxisValue (Variables|Input|GetTurnRateGamepad) (Utilities|Time|GetWorldDeltaSeconds))))

(event Input|AxisEvents|InputAxisTurnRight/LeftMouse
  (params (AxisValue :type Float%20%28single-precision%29))
  ;[0.05098 0.05098 0.05098] Camera - Mouse
  (Pawn|Input|AddControllerYawInput AxisValue))

(event Input|AxisEvents|InputAxisLookUp/DownMouse
  (params (AxisValue :type Float%20%28single-precision%29))
  ;[0.05098 0.05098 0.05098] Camera - Mouse
  (Pawn|Input|AddControllerPitchInput AxisValue))

(event Input|AxisEvents|InputAxisLookUp/DownGamepad
  (params (AxisValue :type Float%20%28single-precision%29))
  ;[0.05098 0.05098 0.05098] Camera - Gamepad
  (Pawn|Input|AddControllerPitchInput (* AxisValue (Variables|Input|GetTurnRateGamepad) (Utilities|Time|GetWorldDeltaSeconds))))

(event Input|AxisEvents|InputAxisMoveRight/Left
  (params (AxisValue :type Float%20%28single-precision%29))
  (bind _returnvalue (Pawn|GetControlRotation :!class /Script/Engine.Pawn))
  ;[0.05098 0.05098 0.05098] Movement
  (Pawn|Input|AddMovementInput (Math|Vector|GetRightVector (Math|Rotator|MakeRotator (.roll _returnvalue) 0.0 (.yaw _returnvalue))) AxisValue false))

(event Input|KeyboardEvents|C
  (params (Key :type Key%20Structure :default "None"))
  ;[0.05098 0.05098 0.05098] Jumping
  (:Pressed
    (Character|Crouch))
  (:Released
    (Character|UnCrouch)))

(event Input|TouchEvents|InputTouch
  (params (Location :type Vector) (FingerIndex :type ETouchIndex%20Enum))
  ;[0.05098 0.05098 0.05098] Jumping
  (:Pressed
    (if (Class|NavMovementComponent|IsFlying (Variables|Character|GetCharacterMovement))
      (CallFunction|GetOffLadder -5e+01))
    (Character|Jump))
  (:Released
    (Character|StopJumping)))

(fn ConstructionScript
  (Variables|Default|SetcameraDefaultTransform (Transformation|GetRelativeTransform (Variables|Camera|GetFollowCamera))))

(fn GetOffLadder
  (params (launchForce :type Float%20%28double-precision%29))
  (bind _returnvalue (Transformation|GetActorForwardVector))
  (bind _returnvalue_2 (* _returnvalue launchForce))
  (Character|LaunchCharacter (Math|Vector|MakeVector (.x _returnvalue_2) (.y _returnvalue_2) 0.0) false false))