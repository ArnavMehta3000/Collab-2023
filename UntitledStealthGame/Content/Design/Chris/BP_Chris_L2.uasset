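; BP_Chris_L2 is a child Blueprint that defines a set of spawn points for enemies, gadgets and keys.
; Its Initialize event runs three init events, one for each category.
; Each passes its named spawn references to the matching AI, gadget or key spawn point function.
; The construction script only calls the parent's.
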(event Custom|InitAiSpawns
  (CallFunction|ToAiSpawnPoint (Variables|Default|GetEnemySpawn))
  (CallFunction|ToAiSpawnPoint (Variables|Default|GetEnemySpawn1))
  (CallFunction|ToAiSpawnPoint (Variables|Default|GetEnemySpawn2))
  (CallFunction|ToAiSpawnPoint (Variables|Default|GetEnemySpawn3))
  (CallFunction|ToAiSpawnPoint (Variables|Default|GetEnemySpawn4))
  (CallFunction|ToAiSpawnPoint (Variables|Default|GetEnemySpawn5))
  (CallFunction|ToAiSpawnPoint (Variables|Default|GetEnemySpawn6))
  (CallFunction|ToAiSpawnPoint (Variables|Default|GetEnemySpawn7))
  (CallFunction|ToAiSpawnPoint (Variables|Default|GetEnemySpawn8))
  (CallFunction|ToAiSpawnPoint (Variables|Default|GetEnemySpawn9))
  (CallFunction|ToAiSpawnPoint (Variables|Default|GetEnemySpawn10))
  (CallFunction|ToAiSpawnPoint (Variables|Default|GetEnemySpawn11)))

(event Custom|InitKeySpawns
  (CallFunction|ToKeySpawnPoint (Variables|Default|GetKeySpawn))
  (CallFunction|ToKeySpawnPoint (Variables|Default|GetKeySpawn1))
  (CallFunction|ToKeySpawnPoint (Variables|Default|GetKeySpawn2)))

(event Custom|InitGadgetSpawns
  (CallFunction|ToGadgetSpawnPoint (Variables|Default|GetGadgetSpawn1))
  (CallFunction|ToGadgetSpawnPoint (Variables|Default|GetGadgetSpawn2))
  (CallFunction|ToGadgetSpawnPoint (Variables|Default|GetGadgetSpawn3))
  (CallFunction|ToGadgetSpawnPoint (Variables|Default|GetGadgetSpawn4))
  (CallFunction|ToGadgetSpawnPoint (Variables|Default|GetGadgetSpawn5)))

(event EventInitialize
  (CallFunction|InitAiSpawns)
  (CallFunction|InitGadgetSpawns)
  (CallFunction|InitKeySpawns))

(fn ConstructionScript
  (|CallParentFunction))