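; BP_Lemarr_I1_Backup is a Lemarr design Blueprint that registers spawn points for enemies, gadgets and keys.
; Its Initialize event runs three sub-events, one per spawn category.
; Each passes its hand-listed spawn point variables individually to ToAiSpawnPoint, ToGadgetSpawnPoint or ToKeySpawnPoint.
; BeginPlay, overlap and Tick are disabled, and the construction script only calls its parent.
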(event Custom|InitAiSpawns
  (CallFunction|ToAiSpawnPoint (Variables|Default|GetEnemySpawnPoint))
  (CallFunction|ToAiSpawnPoint (Variables|Default|GetEnemySpawnPoint1))
  (CallFunction|ToAiSpawnPoint (Variables|Default|GetEnemySpawnPoint2))
  (CallFunction|ToAiSpawnPoint (Variables|Default|GetEnemySpawnPoint3))
  (CallFunction|ToAiSpawnPoint (Variables|Default|GetEnemySpawnPoint4))
  (CallFunction|ToAiSpawnPoint (Variables|Default|GetEnemySpawnPoint5))
  (CallFunction|ToAiSpawnPoint (Variables|Default|GetEnemySpawnPoint6))
  (CallFunction|ToAiSpawnPoint (Variables|Default|GetEnemySpawnPoint7))
  (CallFunction|ToAiSpawnPoint (Variables|Default|GetEnemySpawnPoint8))
  (CallFunction|ToAiSpawnPoint (Variables|Default|GetEnemySpawnPoint9))
  (CallFunction|ToAiSpawnPoint (Variables|Default|GetEnemySpawnPoint10))
  (CallFunction|ToAiSpawnPoint (Variables|Default|GetEnemySpawnPoint11))
  (CallFunction|ToAiSpawnPoint (Variables|Default|GetEnemySpawnPoint12))
  (CallFunction|ToAiSpawnPoint (Variables|Default|GetEnemySpawnPoint13))
  (CallFunction|ToAiSpawnPoint (Variables|Default|GetEnemySpawnPoint14))
  (CallFunction|ToAiSpawnPoint (Variables|Default|GetEnemySpawnPoint15))
  (CallFunction|ToAiSpawnPoint (Variables|Default|GetEnemySpawnPoint16))
  (CallFunction|ToAiSpawnPoint (Variables|Default|GetEnemySpawnPoint17))
  (CallFunction|ToAiSpawnPoint (Variables|Default|GetEnemySpawnPoint18))
  (CallFunction|ToAiSpawnPoint (Variables|Default|GetEnemySpawnPoint19)))

(event Custom|InitKeySpawns
  (CallFunction|ToKeySpawnPoint (Variables|Default|GetKeySpawnPoint))
  (CallFunction|ToKeySpawnPoint (Variables|Default|GetKeySpawnPoint1))
  (CallFunction|ToKeySpawnPoint (Variables|Default|GetKeySpawnPoint2))
  (CallFunction|ToKeySpawnPoint (Variables|Default|GetKeySpawnPoint3)))

(event Custom|InitGadgetSpawns
  (CallFunction|ToGadgetSpawnPoint (Variables|Default|GetGadgetSpawnPoint))
  (CallFunction|ToGadgetSpawnPoint (Variables|Default|GetGadgetSpawnPoint1))
  (CallFunction|ToGadgetSpawnPoint (Variables|Default|GetGadgetSpawnPoint2))
  (CallFunction|ToGadgetSpawnPoint (Variables|Default|GetGadgetSpawnPoint3))
  (CallFunction|ToGadgetSpawnPoint (Variables|Default|GetGadgetSpawnPoint4))
  (CallFunction|ToGadgetSpawnPoint (Variables|Default|GetGadgetSpawnPoint5))
  (CallFunction|ToGadgetSpawnPoint (Variables|Default|GetGadgetSpawnPoint6)))

(event EventBeginPlay
  (|CallParentFunction) ; This node is disabled and will not be called.\nDrag off pins to build functionality.
)

(event Collision|EventActorBeginOverlap
  (params (OtherActor :type Actor%20Object%20Reference))
  (|CallParentFunction OtherActor) ; This node is disabled and will not be called.\nDrag off pins to build functionality.
)

(event EventTick
  (params (DeltaSeconds :type Float%20%28single-precision%29))
  (|CallParentFunction DeltaSeconds) ; This node is disabled and will not be called.\nDrag off pins to build functionality.
)

(event EventInitialize
  (CallFunction|InitAiSpawns)
  (CallFunction|InitGadgetSpawns)
  (CallFunction|InitKeySpawns))

(fn ConstructionScript
  (|CallParentFunction))