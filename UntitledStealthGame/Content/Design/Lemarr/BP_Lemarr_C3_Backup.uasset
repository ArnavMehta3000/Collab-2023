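; BP_Lemarr_C3_Backup is a level-piece Blueprint, apparently a backup, that sets up spawn points for AI enemies, gadgets and keys.
; Initialize runs one init event per category, each passing its hand-listed spawn point references to the matching ToAiSpawnPoint, ToGadgetSpawnPoint or ToKeySpawnPoint helper.
; The helpers are not defined in this Blueprint, and the construction script only calls its parent.
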(event Custom|IntAISpawns
  (CallFunction|ToAiSpawnPoint (Variables|Default|GetEnemySpawnPoint))
  (CallFunction|ToAiSpawnPoint (Variables|Default|GetEnemySpawnPoint1))
  (CallFunction|ToAiSpawnPoint (Variables|Default|GetEnemySpawnPoint2))
  (CallFunction|ToAiSpawnPoint (Variables|Default|GetEnemySpawnPoint3))
  (CallFunction|ToAiSpawnPoint (Variables|Default|GetEnemySpawnPoint4))
  (CallFunction|ToAiSpawnPoint (Variables|Default|GetEnemySpawnPoint5))
  (CallFunction|ToAiSpawnPoint (Variables|Default|GetEnemySpawnPoint6))
  (CallFunction|ToAiSpawnPoint (Variables|Default|GetEnemySpawnPoint7))
  (CallFunction|ToAiSpawnPoint (Variables|Default|GetEnemySpawnPoint8))
  (CallFunction|ToAiSpawnPoint (Variables|Default|GetEnemySpawnPoint9))
  (CallFunction|ToAiSpawnPoint (Variables|Default|GetEnemySpawnPoint10))
  (CallFunction|ToAiSpawnPoint (Variables|Default|GetEnemySpawnPoint11))
  (CallFunction|ToAiSpawnPoint (Variables|Default|GetEnemySpawnPoint12))
  (CallFunction|ToAiSpawnPoint (Variables|Default|GetEnemySpawnPoint13))
  (CallFunction|ToAiSpawnPoint (Variables|Default|GetEnemySpawnPoint14))
  (CallFunction|ToAiSpawnPoint (Variables|Default|GetEnemySpawnPoint15))
  (CallFunction|ToAiSpawnPoint (Variables|Default|GetEnemySpawnPoint16))
  (CallFunction|ToAiSpawnPoint (Variables|Default|GetEnemySpawnPoint17))
  (CallFunction|ToAiSpawnPoint (Variables|Default|GetEnemySpawnPoint18))
  (CallFunction|ToAiSpawnPoint (Variables|Default|GetEnemySpawnPoint19))
  (CallFunction|ToAiSpawnPoint (Variables|Default|GetEnemySpawnPoint20))
  (CallFunction|ToAiSpawnPoint (Variables|Default|GetEnemySpawnPoint21))
  (CallFunction|ToAiSpawnPoint (Variables|Default|GetEnemySpawnPoint22)))

(event Custom|IntGadgetSpawns
  (CallFunction|ToGadgetSpawnPoint (Variables|Default|GetGadgetSpawnPoint))
  (CallFunction|ToGadgetSpawnPoint (Variables|Default|GetGadgetSpawnPoint1))
  (CallFunction|ToGadgetSpawnPoint (Variables|Default|GetGadgetSpawnPoint2))
  (CallFunction|ToGadgetSpawnPoint (Variables|Default|GetGadgetSpawnPoint3))
  (CallFunction|ToGadgetSpawnPoint (Variables|Default|GetGadgetSpawnPoint4))
  (CallFunction|ToGadgetSpawnPoint (Variables|Default|GetGadgetSpawnPoint5))
  (CallFunction|ToGadgetSpawnPoint (Variables|Default|GetGadgetSpawnPoint6))
  (CallFunction|ToGadgetSpawnPoint (Variables|Default|GetGadgetSpawnPoint7))
  (CallFunction|ToGadgetSpawnPoint (Variables|Default|GetGadgetSpawnPoint8))
  (CallFunction|ToGadgetSpawnPoint (Variables|Default|GetGadgetSpawnPoint9))
  (CallFunction|ToGadgetSpawnPoint (Variables|Default|GetGadgetSpawnPoint10))
  (CallFunction|ToGadgetSpawnPoint (Variables|Default|GetGadgetSpawnPoint11)))

(event Custom|IntKeySpawns
  (CallFunction|ToKeySpawnPoint (Variables|Default|GetKeySpawnPoint))
  (CallFunction|ToKeySpawnPoint (Variables|Default|GetKeySpawnPoint1))
  (CallFunction|ToKeySpawnPoint (Variables|Default|GetKeySpawnPoint2))
  (CallFunction|ToKeySpawnPoint (Variables|Default|GetKeySpawnPoint3)))

(event EventInitialize
  (CallFunction|IntAISpawns)
  (CallFunction|IntGadgetSpawns)
  (CallFunction|IntKeySpawns))

(fn ConstructionScript
  (|CallParentFunction))