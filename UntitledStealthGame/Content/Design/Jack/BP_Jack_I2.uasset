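; BP_Jack_I2 is a level-piece Blueprint that supplies climb zones and spawn points for AI, gadgets and keys.
; Overlap begin and end on four box components start and stop climbing for the overlapping actor.
; Initialize runs three setup events that pass hand-placed location components to the AI, gadget and key spawn-point conversion functions.
; The construction script only calls the parent's.
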(event OnComponentBeginOverlap(Box_0)
  (params (OverlappedComponent :type Primitive%20Component%20Object%20Reference) (OtherActor :type Actor%20Object%20Reference) (OtherComp :type Primitive%20Component%20Object%20Reference) (OtherBodyIndex :type Integer) (bFromSweep :type Boolean) (SweepResult :type Hit%20Result%20Structure%20%28by%20ref%29))
  (CallFunction|OnTryStartClimb OtherActor))

(event OnComponentEndOverlap(Box_0)
  (params (OverlappedComponent :type Primitive%20Component%20Object%20Reference) (OtherActor :type Actor%20Object%20Reference) (OtherComp :type Primitive%20Component%20Object%20Reference) (OtherBodyIndex :type Integer))
  (CallFunction|OnTryStopClimb OtherActor))

(event OnComponentBeginOverlap(Box1)
  (params (OverlappedComponent :type Primitive%20Component%20Object%20Reference) (OtherActor :type Actor%20Object%20Reference) (OtherComp :type Primitive%20Component%20Object%20Reference) (OtherBodyIndex :type Integer) (bFromSweep :type Boolean) (SweepResult :type Hit%20Result%20Structure%20%28by%20ref%29))
  (CallFunction|OnTryStartClimb OtherActor))

(event OnComponentEndOverlap(Box1)
  (params (OverlappedComponent :type Primitive%20Component%20Object%20Reference) (OtherActor :type Actor%20Object%20Reference) (OtherComp :type Primitive%20Component%20Object%20Reference) (OtherBodyIndex :type Integer))
  (CallFunction|OnTryStopClimb OtherActor))

(event OnComponentBeginOverlap(Box2)
  (params (OverlappedComponent :type Primitive%20Component%20Object%20Reference) (OtherActor :type Actor%20Object%20Reference) (OtherComp :type Primitive%20Component%20Object%20Reference) (OtherBodyIndex :type Integer) (bFromSweep :type Boolean) (SweepResult :type Hit%20Result%20Structure%20%28by%20ref%29))
  (CallFunction|OnTryStartClimb OtherActor))

(event OnComponentEndOverlap(Box2)
  (params (OverlappedComponent :type Primitive%20Component%20Object%20Reference) (OtherActor :type Actor%20Object%20Reference) (OtherComp :type Primitive%20Component%20Object%20Reference) (OtherBodyIndex :type Integer))
  (CallFunction|OnTryStopClimb OtherActor))

(event OnComponentBeginOverlap(Box3)
  (params (OverlappedComponent :type Primitive%20Component%20Object%20Reference) (OtherActor :type Actor%20Object%20Reference) (OtherComp :type Primitive%20Component%20Object%20Reference) (OtherBodyIndex :type Integer) (bFromSweep :type Boolean) (SweepResult :type Hit%20Result%20Structure%20%28by%20ref%29))
  (CallFunction|OnTryStartClimb OtherActor))

(event OnComponentEndOverlap(Box3)
  (params (OverlappedComponent :type Primitive%20Component%20Object%20Reference) (OtherActor :type Actor%20Object%20Reference) (OtherComp :type Primitive%20Component%20Object%20Reference) (OtherBodyIndex :type Integer))
  (CallFunction|OnTryStopClimb OtherActor))

(event Custom|InitAISpawn
  (CallFunction|ToAiSpawnPoint (Variables|Default|GetEnemySpawnLocation))
  (CallFunction|ToAiSpawnPoint (Variables|Default|GetEnemySpawnLocation1))
  (CallFunction|ToAiSpawnPoint (Variables|Default|GetEnemySpawnLocation2))
  (CallFunction|ToAiSpawnPoint (Variables|Default|GetEnemySpawnLocation3))
  (CallFunction|ToAiSpawnPoint (Variables|Default|GetEnemySpawnLocation4))
  (CallFunction|ToAiSpawnPoint (Variables|Default|GetEnemySpawnLocation5))
  (CallFunction|ToAiSpawnPoint (Variables|Default|GetEnemySpawnLocation6))
  (CallFunction|ToAiSpawnPoint (Variables|Default|GetEnemySpawnLocation7))
  (CallFunction|ToAiSpawnPoint (Variables|Default|GetEnemySpawnLocation8))
  (CallFunction|ToAiSpawnPoint (Variables|Default|GetEnemySpawnLocation9))
  (CallFunction|ToAiSpawnPoint (Variables|Default|GetEnemySpawnLocation10))
  (CallFunction|ToAiSpawnPoint (Variables|Default|GetEnemySpawnLocation11))
  (CallFunction|ToAiSpawnPoint (Variables|Default|GetEnemySpawnLocation12))
  (CallFunction|ToAiSpawnPoint (Variables|Default|GetEnemySpawnLocation13))
  (CallFunction|ToAiSpawnPoint (Variables|Default|GetEnemySpawnLocation14))
  (CallFunction|ToAiSpawnPoint (Variables|Default|GetEnemySpawnLocation15))
  (CallFunction|ToAiSpawnPoint (Variables|Default|GetEnemySpawnLocation16)))

(event Custom|InitGadgetSpawn
  (CallFunction|ToGadgetSpawnPoint (Variables|Default|GetGadgetSpawnLocation))
  (CallFunction|ToGadgetSpawnPoint (Variables|Default|GetGadgetSpawnLocation1))
  (CallFunction|ToGadgetSpawnPoint (Variables|Default|GetGadgetSpawnLocation2))
  (CallFunction|ToGadgetSpawnPoint (Variables|Default|GetGadgetSpawnLocation3))
  (CallFunction|ToGadgetSpawnPoint (Variables|Default|GetGadgetSpawnLocation4))
  (CallFunction|ToGadgetSpawnPoint (Variables|Default|GetGadgetSpawnLocation5))
  (CallFunction|ToGadgetSpawnPoint (Variables|Default|GetGadgetSpawnLocation6))
  (CallFunction|ToGadgetSpawnPoint (Variables|Default|GetGadgetSpawnLocation7))
  (CallFunction|ToGadgetSpawnPoint (Variables|Default|GetGadgetSpawnLocation8))
  (CallFunction|ToGadgetSpawnPoint (Variables|Default|GetGadgetSpawnLocation9)))

(event Custom|InitKeySpawn
  (CallFunction|ToKeySpawnPoint (Variables|Default|GetKeySpawnLocation))
  (CallFunction|ToKeySpawnPoint (Variables|Default|GetKeySpawnLocation1))
  (CallFunction|ToKeySpawnPoint (Variables|Default|GetKeySpawnLocation2)))

(event EventInitialize
  (CallFunction|InitAISpawn)
  (CallFunction|InitGadgetSpawn)
  (CallFunction|InitKeySpawn))

(fn ConstructionScript
  (|CallParentFunction))