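; BP_Daniel_L4 is a level Blueprint asset that sets up the spawn points for enemies, gadgets and keys.
; Initialize runs three init events, one per category.
; Each event passes its numbered spawn point references, one at a time, to the matching ToAiSpawnPoint, ToGadgetSpawnPoint or ToKeySpawnPoint call.
; The spawning logic itself is not defined here, and the construction script is empty.
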(event Custom|InitAiSpawn
  (CallFunction|ToAiSpawnPoint (Variables|Default|GetEnemySpawnPoint))
  (CallFunction|ToAiSpawnPoint (Variables|Default|GetEnemySpawnPoint1))
  (CallFunction|ToAiSpawnPoint (Variables|Default|GetEnemySpawnPoint2))
  (CallFunction|ToAiSpawnPoint (Variables|Default|GetEnemySpawnPoint3))
  (CallFunction|ToAiSpawnPoint (Variables|Default|GetEnemySpawnPoint4))
  (CallFunction|ToAiSpawnPoint (Variables|Default|GetEnemySpawnPoint5))
  (CallFunction|ToAiSpawnPoint (Variables|Default|GetEnemySpawnPoint6))
  (CallFunction|ToAiSpawnPoint (Variables|Default|GetEnemySpawnPoint7))
  (CallFunction|ToAiSpawnPoint (Variables|Default|GetEnemySpawnPoint8))
  (CallFunction|ToAiSpawnPoint (Variables|Default|GetEnemySpawnPoint9))
  (CallFunction|ToAiSpawnPoint (Variables|Default|GetEnemySpawnPoint10))
  (CallFunction|ToAiSpawnPoint (Variables|Default|GetEnemySpawnPoint11))
  (CallFunction|ToAiSpawnPoint (Variables|Default|GetEnemySpawnPoint12))
  (CallFunction|ToAiSpawnPoint (Variables|Default|GetEnemySpawnPoint13))
  (CallFunction|ToAiSpawnPoint (Variables|Default|GetEnemySpawnPoint14)))

(event Custom|InitGadgetSpawn
  (CallFunction|ToGadgetSpawnPoint (Variables|Default|GetGadgetSpawnPoint))
  (CallFunction|ToGadgetSpawnPoint (Variables|Default|GetGadgetSpawnPoint1))
  (CallFunction|ToGadgetSpawnPoint (Variables|Default|GetGadgetSpawnPoint2))
  (CallFunction|ToGadgetSpawnPoint (Variables|Default|GetGadgetSpawnPoint3))
  (CallFunction|ToGadgetSpawnPoint (Variables|Default|GetGadgetSpawnPoint4))
  (CallFunction|ToGadgetSpawnPoint (Variables|Default|GetGadgetSpawnPoint5))
  (CallFunction|ToGadgetSpawnPoint (Variables|Default|GetGadgetSpawnPoint6)))

(event Custom|InitKeySpawn
  (CallFunction|ToKeySpawnPoint (Variables|Default|GetKeySpawnPoint))
  (CallFunction|ToKeySpawnPoint (Variables|Default|GetKeySpawnPoint1))
  (CallFunction|ToKeySpawnPoint (Variables|Default|GetKeySpawnPoint2)))

(event EventInitialize
  (CallFunction|InitAiSpawn)
  (CallFunction|InitGadgetSpawn)
  (CallFunction|InitKeySpawn))

(fn ConstructionScript)