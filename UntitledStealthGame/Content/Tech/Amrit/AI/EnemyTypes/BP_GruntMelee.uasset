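; BP_GruntMelee is a melee grunt enemy Blueprint, still at a placeholder stage.
; It sets its EnemyType on BeginPlay and exposes it through GetEnemyType, while Attack only prints a debug message.
; Tick runs a debug-drawn sphere trace on the Camera channel at the mesh location, but nothing uses the result.
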(event EventTick
  (params (DeltaSeconds :type Float%20%28single-precision%29))
  (bind _mesh (Variables|Character|GetMesh))
  (bind _returnvalue (Transformation|GetWorldLocation _mesh))
  (Collision|SphereTraceByChannel _returnvalue _returnvalue 1.5e+02 "TraceTypeQuery2" false 0 "ForDuration" true "(R=1.000000,G=0.000000,B=0.000000,A=1.000000)" "(R=0.000000,G=1.000000,B=0.000000,A=1.000000)" 0.1))

(event Collision|EventActorBeginOverlap
  (params (OtherActor :type Actor%20Object%20Reference))
  (|CallParentFunction OtherActor) ; This node is disabled and will not be called.\nDrag off pins to build functionality.
)

(event EventAttack
  (Development|PrintString "I'm hitting you"))

(event EventBeginPlay
  (Variables|Default|SetEnemyType "NewEnumerator1"))

(fn ConstructionScript
  (|CallParentFunction))

(fn GetEnemyType
  (return (Variables|Default|GetEnemyType)))