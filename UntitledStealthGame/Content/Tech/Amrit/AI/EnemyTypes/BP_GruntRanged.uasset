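; BP_GruntRanged is a ranged grunt enemy Blueprint that can take cover and shoot the player.
; BeginPlay sets its EnemyType without calling the parent, and GetEnemyType returns that value.
; EnterCover flags it as in cover, crouches and prints a debug message.
; Attack draws a debug line trace from Firepoint to the player, then applies fixed damage regardless of the trace result.
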(event Custom|Enter%20Cover
  (Variables|Default|SetIsInCover true)
  (Character|Crouch)
  (Development|PrintString "IM IN COVER"))

(event Collision|EventActorBeginOverlap
  (params (OtherActor :type Actor%20Object%20Reference)))

(event EventTick
  (params (DeltaSeconds :type Float%20%28single-precision%29)))

(event EventAttack
  (Collision|LineTraceByChannel (Transformation|GetWorldLocation (Variables|Default|GetFirepoint)) (Transformation|GetActorLocation (Game|GetPlayerCharacter 0)) "TraceTypeQuery2" false 0 "ForDuration" true "(R=1.000000,G=0.000000,B=0.000000,A=1.000000)" "(R=0.000000,G=1.000000,B=0.000000,A=1.000000)" 2.0)
  (Game|Damage|ApplyDamage (Game|GetPlayerCharacter 0) 5e+01 0 0))

(event EventBeginPlay
  (Variables|Default|SetEnemyType "NewEnumerator2"))

(fn ConstructionScript
  (|CallParentFunction))

(fn GetEnemyType
  (return (Variables|Default|GetEnemyType)))