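; BP_Sniper is an enemy type Blueprint for a sniper, with placeholder attack logic.
; On BeginPlay it sets its EnemyType enum, which GetEnemyType returns.
; Its Attack event runs a debug-drawn Camera-channel line trace from its mesh to player 0's character and prints "BAM!".
; The trace result is unused, so the attack applies no damage.
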(event Collision|EventActorBeginOverlap
  (params (OtherActor :type Actor%20Object%20Reference))
  (|CallParentFunction OtherActor) ; This node is disabled and will not be called.\nDrag off pins to build functionality.
)

(event EventTick
  (params (DeltaSeconds :type Float%20%28single-precision%29))
  (|CallParentFunction DeltaSeconds) ; This node is disabled and will not be called.\nDrag off pins to build functionality.
)

(event EventAttack
  (Collision|LineTraceByChannel (Transformation|GetWorldLocation (Variables|Character|GetMesh)) (Transformation|GetActorLocation (Game|GetPlayerCharacter 0)) "TraceTypeQuery2" false 0 "ForDuration" true "(R=1.000000,G=0.000000,B=0.000000,A=1.000000)" "(R=0.000000,G=1.000000,B=0.000000,A=1.000000)" 2.0)
  (Development|PrintString "BAM!"))

(event EventBeginPlay
  (Variables|Default|SetEnemyType "NewEnumerator3"))

(fn ConstructionScript
  (|CallParentFunction))

(fn GetEnemyType
  (return (Variables|Default|GetEnemyType)))