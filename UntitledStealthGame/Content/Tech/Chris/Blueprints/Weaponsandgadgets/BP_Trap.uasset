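; BP_Trap is a gadget that temporarily immobilizes AI characters that step into it.
; When its mesh hits a BP_NewRoomBase actor, the mesh switches to static mobility, fixing it in place.
; A sphere overlap with an AI_CharacterBase disables that character's movement, then after a short delay restores it in falling mode and destroys the trap.
; The construction script assigns its gadget type.
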(event OnComponentBeginOverlap(Sphere)
  (params (OverlappedComponent :type Primitive%20Component%20Object%20Reference) (OtherActor :type Actor%20Object%20Reference) (OtherComp :type Primitive%20Component%20Object%20Reference) (OtherBodyIndex :type Integer) (bFromSweep :type Boolean) (SweepResult :type Hit%20Result%20Structure%20%28by%20ref%29))
  (bind _asai_character_base (Utilities|Casting|CastToAI_CharacterBase OtherActor))
  (Pawn|Components|CharacterMovement|DisableMovement (Variables|/Script/Engine.Character|GetCharacterMovement _asai_character_base))
  (Utilities|FlowControl|Delay 4.0)
  (Pawn|Components|CharacterMovement|SetMovementMode (Variables|/Script/Engine.Character|GetCharacterMovement _asai_character_base) "MOVE_Falling" 0)
  (Components|DestroyComponent (Variables|Default|GetBaseMesh))
  (Actor|DestroyActor))

(event OnComponentHit(BaseMesh)
  (params (HitComponent :type Primitive%20Component%20Object%20Reference) (OtherActor :type Actor%20Object%20Reference) (OtherComp :type Primitive%20Component%20Object%20Reference) (NormalImpulse :type Vector :default "0, 0, 0") (Hit :type Hit%20Result%20Structure%20%28by%20ref%29))
  (Utilities|Casting|CastToBP_NewRoomBase OtherActor)
  (Transformation|SetMobility (Variables|Default|GetBaseMesh) "Static"))

(event EventBeginPlay
  (|CallParentFunction) ; This node is disabled and will not be called.\nDrag off pins to build functionality.
)

(event Collision|EventActorBeginOverlap
  (params (OtherActor :type Actor%20Object%20Reference)))

(event EventTick
  (params (DeltaSeconds :type Float%20%28single-precision%29)))

(fn ConstructionScript
  (Variables|Default|SetgadgetType "NewEnumerator5"))