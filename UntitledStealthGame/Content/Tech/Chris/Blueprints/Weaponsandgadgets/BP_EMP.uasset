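; EMP gadget actor that temporarily immobilises AI characters around it.
; Two seconds after BeginPlay it runs a debug-drawn multi sphere trace on the Camera channel and deactivates the CharacterMovement of each AI_CharacterBase hit.
; A Delay inside the loop precedes reactivation and self-destruction, so only the last cast character is reactivated and the actor persists when none is hit.
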(event EventBeginPlay
  (bind _self self)
  (bind _returnvalue (Transformation|GetActorLocation _self))
  (Utilities|FlowControl|Delay 2.0)
  (bind _outhits (Collision|MultiSphereTraceByChannel _returnvalue _returnvalue 5e+02 "TraceTypeQuery2" false 0 "ForDuration"))
  (for _array_element _outhits
    (bind _asai_character_base (Utilities|Casting|CastToAI_CharacterBase (.HitActor (Collision|BreakHitResult _array_element))))
    (Components|Activation|Deactivate (Variables|/Script/Engine.Character|GetCharacterMovement _asai_character_base))
    (Utilities|FlowControl|Delay 5.0)
    (Components|Activation|Activate (Variables|/Script/Engine.Character|GetCharacterMovement _asai_character_base) false)
    (Actor|DestroyActor)))

(fn ConstructionScript
  (Variables|Default|SetgadgetType "NewEnumerator1"))

(fn SetGadgetType
  (params (gadgetType :type E_GadgetType%20Enum :default "NewEnumerator1")))