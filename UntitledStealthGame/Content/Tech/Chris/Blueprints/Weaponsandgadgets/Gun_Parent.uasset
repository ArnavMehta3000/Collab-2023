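; Parent gun Blueprint for weapons attached to the first-person character, providing shared firing, ammo and reload functions.
; StartShooting and StopShooting toggle IsFiring, which FireBullet uses to choose between a damaging camera line trace and spawning a projectile at the barrel.
; Both paths require ammo, but only the trace consumes it and draws persistent debug lines.
; Reload is unfinished, computing the clip shortfall without refilling.
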(event Custom|StartShooting
  (Variables|Default|SetIsFiring true))

(event Custom|StopShooting
  (Variables|Default|SetIsFiring false))

(fn ConstructionScript)

(fn FireBullet
  (if (Variables|Default|GetIsFiring)
    (bind _asbp_first_person_character (Utilities|Casting|CastToBP_FirstPersonCharacter (Actor|GetParentActor)))
    (if (> (Variables|Default|GetCurrentAmmo) 0)
      (bind _outhit (Collision|LineTraceByChannel (Transformation|GetWorldLocation (Variables|/Game/FirstPerson/Blueprints/BP_FirstPersonCharacter.BP_FirstPersonCharacter_C|GetFirstPersonCamera _asbp_first_person_character)) (+ (Transformation|GetWorldLocation (Variables|/Game/FirstPerson/Blueprints/BP_FirstPersonCharacter.BP_FirstPersonCharacter_C|GetFirstPersonCamera _asbp_first_person_character)) (* (Math|Vector|GetForwardVector (Transformation|GetWorldRotation (Variables|/Game/FirstPerson/Blueprints/BP_FirstPersonCharacter.BP_FirstPersonCharacter_C|GetFirstPersonCamera _asbp_first_person_character))) 1e+03)) "TraceTypeQuery1" false 0 "Persistent"))
      (Math|Integer|DecrementInt (Variables|Default|GetCurrentAmmo)
        (:%20%20
          (Game|Damage|ApplyDamage (.HitActor (Collision|BreakHitResult _outhit)) 1e+01 0 0))))
    (else
      (bind _asbp_first_person_character_2 (Utilities|Casting|CastToBP_FirstPersonCharacter (Actor|GetParentActor)))
      (if (> (Variables|Default|GetCurrentAmmo) 0)
        (Game|SpawnActorfromClass (Variables|Default|GetProjectile) (Math|Transform|MakeTransform (Transformation|GetWorldLocation (Variables|Default|Getbarrel_RefPoint)) (Transformation|GetWorldRotation (Variables|/Game/FirstPerson/Blueprints/BP_FirstPersonCharacter.BP_FirstPersonCharacter_C|GetFirstPersonCamera _asbp_first_person_character_2)) "1.000000,1.000000,1.000000") "Undefined" 0 0)))))

(fn Reload
  (bind _output_get (LocalVariables|SetBulletDifference (- (Variables|Default|GetClipSize) (Variables|Default|GetCurrentAmmo))))
  (if (>= (Variables|Default|GetMaxAmmo) _output_get)
    _))