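; Smoke grenade gadget actor that is thrown along the player's aim and sets off an effect where it comes to rest.
; A custom event applies an impulse to the SmokeBomb component along player 0's control rotation, with no added arc.
; A zero-Delay loop polls its velocity until exactly zero, then spawns a scaled-up emitter at GrenadeCentre, plays a sound and destroys the actor after a delay.
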(event Custom|CustomEvent
  (bind _smoke_bomb (Variables|Default|GetSmoke_Bomb))
  (bind _grenade_centre (Variables|Default|GetGrenade_Centre))
  ;[1 1 1] Without Arc
  (Physics|AddImpulse _smoke_bomb (* (Math|Rotator|GetRotationXVector (Pawn|GetControlRotation (Game|GetPlayerController 0) :!class /Script/Engine.Controller)) "350.000000,350.000000,350.000000") "None" false)
  (if (Class|KismetMathLibrary|EqualExactlyVectorVector (Transformation|GetComponentVelocity _smoke_bomb) "0, 0, 0") :!label _label
    (Effects|SpawnEmitteratLocation 0 (Transformation|GetWorldLocation _grenade_centre) (Transformation|GetWorldRotation _grenade_centre) "5.000000,5.000000,5.000000")
    (Audio|PlaySoundatLocation 0 (Transformation|GetActorLocation) "0, 0, 0" 1.0 1.0 0.0 0 0 0 0)
    (Utilities|FlowControl|Delay 1e+01)
    (Actor|DestroyActor)
    (else
      (Utilities|FlowControl|Delay 0.0)
      (goto _label))))

(fn ConstructionScript)