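; Smoke gadget actor that acts as a thrown grenade, launching itself along the player's view and releasing an emitter effect where it comes to rest.
; BeginPlay applies an impulse to the SmokeBomb component along the first player controller's control rotation, then polls its velocity every tick through a zero-delay loop.
; Once velocity is exactly zero, it spawns a scaled-up emitter at GrenadeCentre, waits a fixed delay, deactivates it and destroys itself.
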(event EventBeginPlay
  (bind _smoke_bomb (Variables|Default|GetSmoke_Bomb))
  (bind _grenade_centre (Variables|Default|GetGrenade-Centre))
  (Physics|AddImpulse _smoke_bomb (* (Math|Rotator|GetRotationXVector (Pawn|GetControlRotation (Game|GetPlayerController 0) :!class /Script/Engine.Controller)) "750.000000,750.000000,750.000000") "None" false)
  (if (Class|KismetMathLibrary|EqualExactlyVectorVector (Transformation|GetComponentVelocity _smoke_bomb) "0, 0, 0") :!label _label
    (bind _returnvalue (Effects|SpawnEmitteratLocation 0 (Transformation|GetWorldLocation _grenade_centre) (Transformation|GetWorldRotation _grenade_centre) "5.000000,5.000000,5.000000"))
    (Utilities|FlowControl|Delay 1e+01)
    (Components|Activation|Deactivate _returnvalue)
    (Actor|DestroyActor)
    (else
      (Utilities|FlowControl|Delay 0.0)
      (goto _label))))

(fn ConstructionScript)