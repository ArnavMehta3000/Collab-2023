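; BP_DoorBase is a keycard-gated double sliding door linking two rooms.
; Initialize casts the room references; overlapping Entry with a keycard opens the destination room and both panels once.
; When IsValid, overlapping End consumes the keycard, updates the player's room reference, closes the previous room, shuts the doors after a delay and invalidates the door.
; MoveL and MoveR timelines drive the panels, playing to open and reversing to close.
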(event OnComponentBeginOverlap(Entry)
  (params (OverlappedComponent :type Primitive%20Component%20Object%20Reference) (OtherActor :type Actor%20Object%20Reference) (OtherComp :type Primitive%20Component%20Object%20Reference) (OtherBodyIndex :type Integer) (bFromSweep :type Boolean) (SweepResult :type Hit%20Result%20Structure%20%28by%20ref%29))
  ;[0 0 0] On Entry Next Room
  (bind _asmasterplayer (Utilities|PlayerCheck OtherActor)
    (:ExecOut
      (if (Variables|/Game/Master/Blueprint/Player/BP_MasterPlayer.BP_MasterPlayer_C|GethasKeycard _asmasterplayer)
        (Utilities|FlowControl|DoOnce false
          (:Completed
            (Default|OpenRoom (Variables|Default|GettoRoom))
            (Utilities|OpenDoors)))))))

(event OnComponentBeginOverlap(End)
  (params (OverlappedComponent :type Primitive%20Component%20Object%20Reference) (OtherActor :type Actor%20Object%20Reference) (OtherComp :type Primitive%20Component%20Object%20Reference) (OtherBodyIndex :type Integer) (bFromSweep :type Boolean) (SweepResult :type Hit%20Result%20Structure%20%28by%20ref%29))
  ;[0 0 0] On Exit Previous Room
  (bind _asmasterplayer (Utilities|Door/PlayerValidCheck OtherActor) ; Check if door can open and hit actor is player
    (:ExecOut
      (Variables|/Game/Master/Blueprint/Player/BP_MasterPlayer.BP_MasterPlayer_C|SethasKeycard _asmasterplayer false)
      (Default|UpdateRoomRef _asmasterplayer (Variables|Default|GettoRoom))
      (Default|CloseRoom (Variables|Default|GetfromRoom))
      (Utilities|FlowControl|Delay 1.0)
      (Utilities|CloseDoors)
      (Variables|Default|SetisValid false))))

(event Custom|CloseDoorRight
  ;[0 0 0] Move Doors
  ;;[0 0 0] Affect Right Door
  (bind _relativepos (Timeline|MoveR Reverse)
    (:Update
      (Transformation|SetRelativeLocation (Variables|Default|GetRightDoor) _relativepos false false))))

(event Custom|OpenDoorRight
  ;[0 0 0] Move Doors
  ;;[0 0 0] Affect Right Door
  (bind _relativepos (Timeline|MoveR Play)
    (:Update
      (Transformation|SetRelativeLocation (Variables|Default|GetRightDoor) _relativepos false false))))

(event Custom|OpenDoorLeft
  ;[0 0 0] Move Doors
  ;;[0 0 0] Affect Left Door
  (bind _relativepos (Timeline|MoveL Play)
    (:Update
      (Transformation|SetRelativeLocation (Variables|Default|GetLeftDoor) _relativepos false false))))

(event Custom|CloseDoorLeft
  ;[0 0 0] Move Doors
  ;;[0 0 0] Affect Left Door
  (bind _relativepos (Timeline|MoveL Reverse)
    (:Update
      (Transformation|SetRelativeLocation (Variables|Default|GetLeftDoor) _relativepos false false))))

(event EventInitialize
  ;[0 0 0] Initialize
  (Variables|Default|SetfromRoom (.AsBP%20New%20Room%20Base (Utilities|Casting|CastToBP_NewRoomBase (Variables|Default|GetcameFromRoom))))
  (Variables|Default|SettoRoom (.AsBP%20New%20Room%20Base (Utilities|Casting|CastToBP_NewRoomBase (Variables|Default|GetgoingToRoom)))))

(fn ConstructionScript)