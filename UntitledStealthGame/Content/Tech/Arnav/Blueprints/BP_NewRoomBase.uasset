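; Base room Blueprint that populates a room with enemies and a keycard when opened and destroys those enemies when closed.
; Helper functions cast child actors into AI, gadget and key spawn-point lists; gadget points are unused here.
; OpenRoom spawns enemies at random AI points until MaxEnemySpawnCount, retrying on CanSpawn failure, then after a short delay spawns and initializes a keycard at a random key point.
; CloseRoom destroys the tracked controllers and characters, leaving the keycard.
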(event Custom|OpenRoom
  (Spawners|SpawnRoomEnemies)
  (Utilities|FlowControl|Delay 0.2)
  (bind _returnvalue (Game|SpawnActorfromClass "/Game/Master/Blueprint/BP_Keycard.BP_Keycard_C" (Math|Transform|MakeTransform (Transformation|GetActorLocation (.OutItem (Utilities|Array|Random (Variables|Default|GetkeySpawnPoints)))) "0, 0, 0" (Math|Conversions|ToVector(Float) 2.0)) "Undefined" self 0))
  (Utilities|IsValid _returnvalue
    (:Is%20Valid
      (Class|IInitable|Initialize(Message) _returnvalue))
    (:Is%20Not%20Valid
      (Development|PrintString "KEY NOT VALID" true true "(R=1.000000,G=0.000000,B=0.103839,A=1.000000)"))))

(fn ConstructionScript)

(fn ToAiSpawnPoint
  (params (childActor :type Child%20Actor%20Component%20Object%20Reference))
  (bind _asbp_ai_spawn_point (Utilities|Casting|CastToBP_AiSpawnPoint (Variables|/Script/Engine.ChildActorComponent|GetChildActor childActor))
    (:then
      (Utilities|Array|Add (Variables|Default|GetaiSpawnPoints) _asbp_ai_spawn_point))
    (:CastFailed
      (Development|PrintString "Failed to cast to Ai key point" true true "(R=1.000000,G=0.000000,B=0.248025,A=1.000000)"))))

(fn ToGadgetSpawnPoint
  (params (childActor :type Child%20Actor%20Component%20Object%20Reference))
  (bind _asbp_gadget_spawn_point (Utilities|Casting|CastToBP_GadgetSpawnPoint (Variables|/Script/Engine.ChildActorComponent|GetChildActor childActor))
    (:then
      (Utilities|Array|Add (Variables|Default|GetgadgetSpawnPoints) _asbp_gadget_spawn_point))
    (:CastFailed
      (Development|PrintString "Failed to cast to gadget spawn point" true true "(R=1.000000,G=0.000000,B=0.248025,A=1.000000)"))))

(fn ToKeySpawnPoint
  (params (childActor :type Child%20Actor%20Component%20Object%20Reference))
  (bind _asbp_key_spawn_point (Utilities|Casting|CastToBP_KeySpawnPoint (Variables|/Script/Engine.ChildActorComponent|GetChildActor childActor))
    (:then
      (Utilities|Array|Add (Variables|Default|GetkeySpawnPoints) _asbp_key_spawn_point))
    (:CastFailed
      (Development|PrintString "Failed to cast to key spawn point" true true "(R=1.000000,G=0.000000,B=0.248025,A=1.000000)"))))

(fn SpawnRoomEnemies
  (bind _aispawnpoints (Variables|Default|GetaiSpawnPoints))
  (bind _outitem (Utilities|Array|Random _aispawnpoints))
  (LocalVariables|Setcount 0)
  (if (not (== (Math|Conversions|ToInteger(Byte) (Variables|Default|GetMaxEnemySpawnCount)) (LocalVariables|Getcount))) :!label _label
    (if (Variables|/Game/Tech/Arnav/Blueprints/BP_AiSpawnPoint.BP_AiSpawnPoint_C|GetcanSpawn _outitem)
      (bind (_character _controller) (Default|SpawnEnemyatPoint _outitem))
      (Utilities|Array|Add (Variables|Default|GetspawnedAI) _character)
      (Utilities|Array|Add (Variables|Default|GetspawnedControllers) _controller)
      (Math|Integer|IncrementInt (LocalVariables|Getcount)
        (:%20%20
          (goto _label)))
      (else
        (goto _label)))))

(fn CloseRoom
  (for _array_element (Variables|Default|GetspawnedControllers)
    (Actor|DestroyActor _array_element))
  (for _array_element_2 (Variables|Default|GetspawnedAI)
    (Actor|DestroyActor _array_element_2)))