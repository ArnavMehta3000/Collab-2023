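; BP_GadgetSpawnPoint is a pickup actor that gives the player an EMP, Sound or Trap gadget.
; SpawnGadgets rolls a random float to choose among the three at roughly equal odds and sets the matching mesh; nothing in this file calls it.
; Overlapping the sphere passes the chosen gadget to the master player through OnPickUp, then destroys the actor, so each instance gives one pickup.
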(event OnComponentBeginOverlap(Sphere)
  (params (OverlappedComponent :type Primitive%20Component%20Object%20Reference) (OtherActor :type Actor%20Object%20Reference) (OtherComp :type Primitive%20Component%20Object%20Reference) (OtherBodyIndex :type Integer) (bFromSweep :type Boolean) (SweepResult :type Hit%20Result%20Structure%20%28by%20ref%29))
  (bind _asbp_master_player (Utilities|ToMasterPlayer OtherActor)
    (:then
      (Default|CallOnPickUp _asbp_master_player (Variables|Default|Getgadget) false)
      (Actor|DestroyActor))))

(fn ConstructionScript)

(fn SpawnGadgets
  (bind _output_get (LocalVariables|SettempNum (Math|Random|RandomFloat)))
  (if (Utilities|IsinRange _output_get 0.0 0.33)
    (Variables|Default|Setgadget "NewEnumerator2")
    (Components|StaticMesh|SetStaticMesh (Variables|Default|GetGadgetMesh) (Utilities|Select :Index (Variables|Default|Getgadget) :NewEnumerator1 "/Game/Art/gameplayassets/Gadgets/EMP/EMP_low.EMP_low" :NewEnumerator2 "/Game/Art/gameplayassets/Gadgets/Sound/Soundgadget.Soundgadget" :NewEnumerator5 "/Game/Art/gameplayassets/Gadgets/Trap/trap.trap") :!label _label)
    (elif (Utilities|IsinRange _output_get 0.33 0.67)
      (Variables|Default|Setgadget "NewEnumerator1")
      (goto _label)
      (elif (Utilities|IsinRange _output_get 0.67 1.0)
        (Variables|Default|Setgadget "NewEnumerator5")
        (goto _label)))))