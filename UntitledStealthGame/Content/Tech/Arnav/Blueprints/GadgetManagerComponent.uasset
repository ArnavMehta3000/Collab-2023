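; Gadget manager component that tracks how many of each gadget type are held, using a map from gadget enum to count.
; ResetCount clears the map and re-seeds all six gadget types at zero, while PickUpGadget and UseGadget increment or decrement a type's count.
; CanUseGadget reports whether a count is above zero, but UseGadget does not check it itself.
; Pickup and use both print debug strings, both labeled "Used Gadget".
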(fn ResetCount
  (bind _gadgetmap (Variables|Default|GetgadgetMap))
  (Utilities|Map|Clear (Variables|Default|GetgadgetMap))
  (Utilities|Map|Add _gadgetmap "NewEnumerator0" 0)
  (Utilities|Map|Add _gadgetmap "NewEnumerator1" 0)
  (Utilities|Map|Add _gadgetmap "NewEnumerator2" 0)
  (Utilities|Map|Add _gadgetmap "NewEnumerator3" 0)
  (Utilities|Map|Add _gadgetmap "NewEnumerator4" 0)
  (Utilities|Map|Add _gadgetmap "NewEnumerator5" 0))

(fn UseGadget
  (params (gadgetType :type E_GadgetType%20Enum :default "NewEnumerator0"))
  (bind _gadgetmap (Variables|Default|GetgadgetMap))
  (bind _result (Math|Integer|DecrementInt (.Value (Utilities|Map|Find _gadgetmap gadgetType)))
    (:%20%20
      (Utilities|Map|Add _gadgetmap gadgetType _result)
      (Development|PrintString (Utilities|String|Append "Used Gadget: " (Utilities|String|EnumtoString gadgetType) "Count: " (Utilities|String|ToString(Integer) _result))))))

(fn CanUseGadget
  (params (gadgetType :type E_GadgetType%20Enum :default "NewEnumerator0"))
  (return (> (.Value (Utilities|Map|Find (Variables|Default|GetgadgetMap) gadgetType)) 0)))

(fn PickUpGadget
  (params (gadgetType :type E_GadgetType%20Enum :default "NewEnumerator0"))
  (bind _gadgetmap (Variables|Default|GetgadgetMap))
  (bind _result (Math|Integer|IncrementInt (.Value (Utilities|Map|Find _gadgetmap gadgetType)))
    (:%20%20
      (Utilities|Map|Add _gadgetmap gadgetType _result)
      (Development|PrintString (Utilities|String|Append "Used Gadget: " (Utilities|String|EnumtoString gadgetType) "Count: " (Utilities|String|ToString(Integer) _result))))))